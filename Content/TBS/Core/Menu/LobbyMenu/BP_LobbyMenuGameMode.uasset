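; Game mode for a two-player TBS lobby menu that accepts a host and one client, kicks extra logins, and relays lord choices and ready states.
; Looping and timeout timers exchange client pings and responses, removing an unresponsive client as a rage quitter and resetting readiness.
; Once both players are ready the host HUD enables Start; a client check then precedes a delayed server travel, cancelled if a player leaves.
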(event Custom|ConnectionChecking_Client
  (bind _controllers (Variables|Default|GetControllers))
  ;[0.6042 0.3519 1 1 32] Checking Connection
  (if (Utilities|Array|IsValidIndex _controllers 1)
    (bind _asbp_lobby_menu_player_controller (Utilities|Casting|CastToBP_LobbyMenuPlayerController (Utilities|Array|Get(acopy) _controllers 1)))
    (Default|ResetTimetoDisconnectCLIENT _asbp_lobby_menu_player_controller)))

(event Custom|ConnectionChecking_Server
  ;[0.6042 0.3519 1 1 32] Checking Connection
  (for (_ _array_index) (Variables|Default|GetControllers)
    (if (!= _array_index 0)
      (CallFunction|RemoveRageQuicker))))

(event Custom|ClearTimers
  ;[0.6042 0.3519 1 1 32] Checking Connection
  (Utilities|Time|ClearandInvalidateTimerbyHandle (Variables|Default|GetTH_ConnectionChecking_Client))
  (Utilities|Time|ClearandInvalidateTimerbyHandle (Variables|Default|GetTH_ConnectionChecking_Server))
  (Utilities|Time|ClearandInvalidateTimerbyHandle (Variables|Default|GetTH_EnteringInGame_Response)))

(event Custom|RemoveRageQuicker
  ;[0.6042 0.3519 1 1 32] Checking Connection
  (CallFunction|ClearTimers)
  (bind _asbp_lobby_menu_player_controller (Utilities|Casting|CastToBP_LobbyMenuPlayerController (Game|GetPlayerController 0)))
  (Default|PlayerHasLeavedSERVER _asbp_lobby_menu_player_controller 0 true true)
  (Variables|Default|SetReadyPlayers 0)
  (Utilities|FlowControl|Delay 0.75)
  (if (not (Utilities|Time|IsTimerActivebyHandle (Variables|Default|GetTH_ConnectionChecking_Client)))
    (Variables|Default|SetControllers (Utilities|Array|MakeArray (Game|GetPlayerController 0)))))

(event Custom|TimeOut_RageQuick
  ;[0.2566 1 0.3366 1 32] Start Game
  (CallFunction|RemoveRageQuicker))

(event EventPlayerIsReadytoStart
  (params (Player :type Player%20Controller%20Object%20Reference))
  ;[0.2566 1 0.3366 1 32] Start Game
  (Math|Integer|IncrementInt (Variables|Default|GetReadyPlayers)
    (:%20%20
      (Class|BPILobbyController|OpponentIsReady(Message) (Utilities|Array|Get(acopy) (Variables|Default|GetControllers) (Utilities|Select :Index (Utilities|Array|FindItem (Variables|Default|GetControllers) Player) :Option%200 1 :Option%201 0)))
      (if (== (Variables|Default|GetReadyPlayers) 2)
        (Class|BPILobbyHUD|EnableStartGameButton(Message) (HUD|GetHUD (Game|GetPlayerController 0)))))))

(event EventDestroyCurrentSession
  ;[0.8935 0.15 1 1 32] Quit Game
  (for (_array_element _array_index) (Variables|Default|GetControllers)
    (bind _asbp_lobby_menu_player_controller (Utilities|Casting|CastToBP_LobbyMenuPlayerController _array_element))
    (Default|ExitCurrentSessionCLIENT _asbp_lobby_menu_player_controller (Utilities|Select :Index _array_index :Option%200 "NewEnumerator0" :Option%201 "NewEnumerator2"))))

(event EventSetNewOpponentLordClass
  (params (Sender :type Controller%20Object%20Reference) (NewLord :type E_LordClasses%20Enum :default "NewEnumerator0"))
  (bind _controllers (Variables|Default|GetControllers))
  ;[0.2502 0.4418 1 1 32] On Player Login
  (if (> (Utilities|Array|Length _controllers) 1)
    (bind _asbp_lobby_menu_player_controller (Utilities|Casting|CastToBP_LobbyMenuPlayerController (Utilities|Array|Get(acopy) _controllers (select (Pawn|IsLocalController Sender) 1 0))))
    (Default|SetNewOpponentLordClassCLIENT _asbp_lobby_menu_player_controller NewLord)))

(event EventPostLogin
  (params (NewPlayer :type Player%20Controller%20Object%20Reference))
  ;[0.2502 0.4418 1 1 32] On Player Login
  (if (< (Utilities|Array|Length (Variables|Default|GetControllers)) 2)
    (Variables|Default|SetPressedButtons 0)
    (Utilities|Array|Add (Variables|Default|GetControllers) NewPlayer)
    (if (== (Utilities|Array|Length (Variables|Default|GetControllers)) 2)
      (Development|PrintString "PLAYER 2 CONNECTED" true true "(R=0.000000,G=1.000000,B=0.208113,A=1.000000)" 5.0)
      (CallFunction|ClearTimers)
      (bind _returnvalue (Utilities|Time|SetTimerbyEvent (EventDispatchers|CreateEvent :!event Custom|ConnectionChecking_Client) 3.0 true))
      (Variables|Default|SetTH_ConnectionChecking_Client _returnvalue)
      (bind _returnvalue_2 (Utilities|Time|SetTimerbyEvent (EventDispatchers|CreateEvent :!event Custom|ConnectionChecking_Server) 2e+01))
      (Variables|Default|SetTH_ConnectionChecking_Server _returnvalue_2))
    (else
      (Utilities|FlowControl|Delay 0.25)
      (Default|KickPlayerCLIENT (.AsBP%20Lobby%20Menu%20Player%20Controller (Utilities|Casting|CastToBP_LobbyMenuPlayerController NewPlayer)) :!label _label)
      (Utilities|FlowControl|Delay 0.25)
      (Utilities|IsValid NewPlayer
        (:Is%20Valid
          (goto _label))))))

(event EventProvideEnteringinGame
  (params (LevelName :type Name :default "None") (EnteringDelay :type Float%20%28single-precision%29))
  ;[0.2566 1 0.3366 1 32] Start Game
  (Variables|Default|SetbEnteringInGame true)
  (CallFunction|ClearTimers)
  (for (_array_element _array_index) (Variables|Default|GetControllers)
    (if (< _array_index 2)
      (bind _asbp_lobby_menu_player_controller (Utilities|Casting|CastToBP_LobbyMenuPlayerController _array_element))
      (Default|StartEnteringinGameCLIENT _asbp_lobby_menu_player_controller)
      (else
        (Default|KickPlayerCLIENT (.AsBP%20Lobby%20Menu%20Player%20Controller (Utilities|Casting|CastToBP_LobbyMenuPlayerController _array_element))))))
  (Utilities|FlowControl|Delay EnteringDelay)
  (if (Variables|Default|GetbEnteringInGame)
    (Development|ExecuteConsoleCommand (Utilities|String|Append "servertravel " (Utilities|String|ToString(Name) LevelName)) (Game|GetPlayerController 0))))

(event EventOnPlayerLeaved
  (params (Player :type Controller%20Object%20Reference))
  ;[0.8935 0.15 1 1 32] Quit Game
  (if (Utilities|Array|ContainsItem (Variables|Default|GetControllers) Player)
    (if (Variables|Default|GetbEnteringInGame)
      (Variables|Default|SetbEnteringInGame false)
      (Class|BPILobbyHUD|PlayAppearanceAnimAfterLeaving(Message) (HUD|GetHUD (Game|GetPlayerController 0))))
    (Utilities|Array|RemoveItem (Variables|Default|GetControllers) Player)
    (Variables|Default|SetReadyPlayers 0)
    (CallFunction|ClearTimers)))

(event EventRemoveInvalidPlayers
  ;[0.8935 0.15 1 1 32] Quit Game
  (for (_array_element _array_index) (Variables|Default|GetControllers)
    (if (!= _array_index 0)
      (Actor|DestroyActor _array_element)
      (Utilities|Array|RemoveIndex (Variables|Default|GetControllers) _array_index))))

(event EventClientIsHereResponse
  ;[0.6042 0.3519 1 1 32] Checking Connection
  (bind _returnvalue (Utilities|Time|SetTimerbyEvent (EventDispatchers|CreateEvent :!event Custom|ConnectionChecking_Server) 2e+01))
  (Variables|Default|SetTH_ConnectionChecking_Server _returnvalue)
  (Development|PrintString "Server: Client Is Here" true true "(R=0.000000,G=1.000000,B=0.187829,A=1.000000)" 5.0))

(event EventCheckCanStart
  ;[0.2566 1 0.3366 1 32] Start Game
  (bind _asbp_lobby_menu_player_controller (Utilities|Casting|CastToBP_LobbyMenuPlayerController (Utilities|Array|Get(acopy) (Variables|Default|GetControllers) 1))
    (:then
      (Default|CheckingfromServerCLIENT _asbp_lobby_menu_player_controller)
      (bind _returnvalue (Utilities|Time|SetTimerbyEvent (delegate Custom|TimeOut_RageQuick) 1e+01))
      (Variables|Default|SetTH_EnteringInGame_Response _returnvalue))
    (:CastFailed
      (CallFunction|RemoveRageQuicker))))

(event EventClientIsHereCanStart
  ;[0.2566 1 0.3366 1 32] Start Game
  (CallFunction|ClearTimers)
  (Class|BPILobbyHUD|StartEnteringinGame(Message) (HUD|GetHUD (Game|GetPlayerController 0))))

(event EventTick
  (params (DeltaSeconds :type Float%20%28single-precision%29))
  (Development|PrintString (Utilities|String|Append "Num of Players: " (Utilities|String|ToString(Integer) (Utilities|Array|Length (Variables|Default|GetControllers))) "   Ready:   " (Utilities|String|ToString(Integer) (Variables|Default|GetReadyPlayers))) true true "(R=0.679362,G=1.000000,B=0.171278,A=1.000000)" 0.0))

(fn ConstructionScript)

(fn GetClientPlayerController
  (return (Utilities|Array|Get(acopy) (Variables|Default|GetControllers) 1)))

(fn GetNumOfPlayers
  (return (Utilities|Array|Length (Variables|Default|GetControllers))))

(fn GetPlayers
  (return (Variables|Default|GetControllers)))

(fn IsPlayerReady
  (params (Player :type Integer))
  (return (== (Variables|Default|GetReadyPlayers) 1)))

(fn IsValidController
  (params (Controller :type Controller%20Object%20Reference))
  (return (Utilities|Array|ContainsItem (Variables|Default|GetControllers) Controller)))