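; BP_LobbyMenuHUD is the lobby menu HUD, which owns the lobby menu widget.
; On BeginPlay it waits briefly, then creates W_LobbyMenuWidget for the first player controller, stores it and adds it to the viewport.
; Its events forward start-button enabling, disabling and the disappearing animation to the widget.
; GetDisappearAnimLength returns the widget's reported time to finish its animations.
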(event EventBeginPlay
  (Utilities|FlowControl|Delay 1.0)
  (bind _returnvalue (UserInterface|CreateWidget "/Game/TBS/UI/Menu/W_LobbyMenuWidget.W_LobbyMenuWidget_C" (Game|GetPlayerController 0)))
  (bind _output_get (Variables|Default|SetW_LobbyMenu _returnvalue))
  (UserInterface|Viewport|AddtoViewport _output_get 0))

(event EventPlayDisappearingAnimation
  (Default|PlayDisappearingAnim (Variables|Default|GetW_LobbyMenu)))

(event EventDisableStartGameButton
  (Default|DisableStartGameButton (Variables|Default|GetW_LobbyMenu)))

(event EventEnableStartGameButton
  (Default|EnableStartGameBtn (Variables|Default|GetW_LobbyMenu)))

(fn ConstructionScript)

(fn GetDisappearAnimLength
  (bind _returnvalue (Default|GetTimetoFinishAnims (Variables|Default|GetW_LobbyMenu)))
  (return _returnvalue))