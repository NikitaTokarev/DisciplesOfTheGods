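; Base Blueprint for timed effects in the turn-based game, with data table-driven definitions and runtime hero effect state.
; InitializeEffect loads the row from RowHandle and stores duration and power in an effect struct.
; Each UpdateEffectState call decrements duration and returns a response with damage from truncated power, text, sound and a finished flag.
; Expiry or manual deactivation clears all stored data, and getters expose the effect's data, name and type.
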(event Custom|InitializeEffect
  (params (Duration :type Integer) (EffectPower :type Float%20%28single-precision%29))
  (bind _rowhandle (Variables|Default|GetRowHandle))
  (bind (_datatable _rowname) (Utilities|Struct|BreakDataTableRowHandle _rowhandle))
  (bind _returnvalue (Utilities|GetDataTableRow _datatable _rowname)
    (:then
      (Variables|Default|SetMainData _returnvalue))
    (:RowNotFound
      _))
  (Variables|Default|SetDuration Duration)
  (Variables|Default|SetEffect%20Power EffectPower)
  (Variables|Default|SetEffectData (Utilities|Struct|MakeS_HeroEffect (Variables|Default|GetRowHandle) 0.0 (Variables|Default|GetDuration) (Variables|Default|GetEffect%20Power))))

(fn UpdateEffectState
  (bind _maindata (Variables|Default|GetMainData))
  (bind (_updatedtext _finishedtext) (Utilities|Struct|BreakS_EffectMain _maindata))
  (bind _result (Math|Integer|DecrementInt (Variables|Default|GetDuration))
    (:%20%20
      (LocalVariables|SetL_Finished (== _result 0))
      (LocalVariables|SetL_Response (Utilities|Struct|MakeS_EffectResponse (Math|Float|Truncate (Variables|Default|GetEffect%20Power)) (select (LocalVariables|GetL_Finished) _finishedtext _updatedtext) (LocalVariables|GetL_Finished) (Utilities|Struct|BreakS_EffectMain (Variables|Default|GetMainData))))
      (Utilities|Struct|SetmembersinS_HeroEffect (Variables|Default|GetEffectData) (Variables|Default|GetDuration))
      (if (LocalVariables|GetL_Finished)
        (TBS|Effects|Inherited|PreparetoRemove))
      (return (LocalVariables|GetL_Response)))))

(fn DeactivateEffect
  (TBS|Effects|Inherited|PreparetoRemove)
  (return))

(fn PreparetoRemove
  (Variables|Default|SetRowHandle "")
  (Variables|Default|SetMainData "")
  (Variables|Default|SetDuration 0)
  (Variables|Default|SetEffect%20Power 0.0)
  (Variables|Default|SetEffectData "")
  (return))

(fn GetEffectData
  (return (Variables|Default|GetEffectData)))

(fn GetMainData
  (return (Variables|Default|GetMainData)))

(fn GetEffectName
  (return (Utilities|Struct|BreakDataTableRowHandle (Variables|Default|GetRowHandle))))

(fn GetEffectType
  (return (Utilities|Struct|BreakS_EffectMain (Variables|Default|GetMainData))))