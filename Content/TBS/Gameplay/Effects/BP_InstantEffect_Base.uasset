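; Base Blueprint for one-shot effects applied to units in the turn-based game.
; Initialization stores the target unit and effect power, then loads the effect's data from DT_EFFECTS through its row handle.
; UpdateEffectState runs the effect if allowed, returns a response built from calculated damage, and always prepares the effect for removal.
; CheckCanBeExecuted (true by default) and the empty ExecuteInstantEffect serve as hooks for child effects.
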(event EventInitializeEffect
  (params (UnitRef :type BP%20Hero%20Base%20Object%20Reference) (Duration :type Integer) (EffectPower :type Float%20%28single-precision%29))
  (Variables|Default|SetUnitRef UnitRef)
  (Variables|Default|SetEffect%20Power EffectPower)
  (bind _returnvalue (Utilities|GetDataTableRow "/Game/TBS/Data/Gameplay/DT_EFFECTS.DT_EFFECTS" (Utilities|Struct|BreakDataTableRowHandle (Variables|Default|GetRowHandle)))
    (:then
      (Variables|Default|SetMainData _returnvalue))))

(fn UpdateEffectState
  (params (Round :type Integer))
  (bind _returnvalue (TBS|Effects|Inherited|CheckCanbeExecuted))
  (if _returnvalue
    (TBS|Effects|Inherited|ExecuteInstantEffect)
    (LocalVariables|SetL_Response (Utilities|Struct|MakeS_EffectResponse (CallFunction|CalculateDamage))))
  (CallFunction|PreparetoRemove)
  (return (LocalVariables|GetL_Response) _returnvalue))

(fn CheckCanbeExecuted
  (return true))

(fn ExecuteInstantEffect)