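; Shock status effect for the turn-based strategy game that lowers the affected unit's initiative by an amount derived from a debuff coefficient.
; On imposition it undoes any stored reduction, recalculates the amount through the unit and applies it as a negative change, so repeat applications do not stack.
; On finish it restores the stored amount, then runs parent removal and clears its values.
; CalculateDecreasingValue is an unimplemented stub.
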(event EventOnEffectImposed
  (if (== (Variables|Default|GetDecreasingValue) -1)
    _
    (else
      (Default|ChangeUnitInitiative (Variables|Default|GetUnitRef) (Variables|Default|GetDecreasingValue))))
  (bind _returnvalue (Default|CalculatePercenttoChangeInitiative (Variables|Default|GetUnitRef) (Variables|Default|GetDebuffCoef)))
  (bind _output_get (Variables|Default|SetDecreasingValue _returnvalue))
  (Default|ChangeUnitInitiative (Variables|Default|GetUnitRef) (* _output_get -1)))

(event EventOnEffectFinished
  (Default|ChangeUnitInitiative (Variables|Default|GetUnitRef) (Variables|Default|GetDecreasingValue))
  (CallFunction|PreparetoRemove))

(fn CalculateDecreasingValue)

(fn PreparetoRemove
  (|CallParentFunction)
  (Variables|Default|SetDebuffCoef 0.0)
  (Variables|Default|SetDecreasingValue 0)
  (return))