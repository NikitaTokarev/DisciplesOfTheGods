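; Shock unit effect for the turn-based game that lowers the affected unit's initiative by a percentage set by DebuffCoef.
; On imposition it undoes any stored change, applies the percentage cut and saves the returned delta, so repeat applications do not stack.
; On finish it reverses that delta as a flat value, and PrepareToRemove clears both the coefficient and stored delta.
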(event EventOnEffectImposed
  (if (== (Variables|Default|GetDecreasingValue) 0)
    _
    (else
      (Default|ChangeUnitInitiative (Variables|Default|GetUnitRef) (Math|Conversions|ToFloat(Integer) (* (Variables|Default|GetDecreasingValue) -1)) false)))
  (bind _returnvalue (Default|ChangeUnitInitiative (Variables|Default|GetUnitRef) (* (Variables|Default|GetDebuffCoef) -1.0) true))
  (Variables|Default|SetDecreasingValue _returnvalue))

(event EventOnEffectFinished
  (Default|ChangeUnitInitiative (Variables|Default|GetUnitRef) (Math|Conversions|ToFloat(Integer) (* (Variables|Default|GetDecreasingValue) -1)) false)
  (|CallParentFunction))

(fn PreparetoRemove
  (|CallParentFunction)
  (Variables|Default|SetDebuffCoef 0.0)
  (Variables|Default|SetDecreasingValue 0)
  (return))