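; Encouragement unit effect for the turn-based game that adjusts a unit's initiative and damage by a percentage coefficient.
; When imposed, it first reverts any previously applied change, then applies BuffCoef as a percentage and stores the resulting deltas so re-imposing does not stack.
; When finished, it subtracts the stored deltas as flat values and calls the parent logic.
; PrepareToRemove calls the parent and resets the coefficient and stored deltas.
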(event EventOnEffectImposed
  (if (== (Variables|Default|GetIncreasingValue_Initiative) 0)
    _
    (else
      (Default|ChangeUnitInitiative (Variables|Default|GetUnitRef) (Math|Conversions|ToFloat(Integer) (* (Variables|Default|GetIncreasingValue_Initiative) -1)) false)))
  (if (== (Variables|Default|GetIncreasingValue_Damage) 0)
    _
    (else
      (Default|ChangeUnitDamage (Variables|Default|GetUnitRef) (Math|Conversions|ToFloat(Integer) (* (Variables|Default|GetIncreasingValue_Damage) -1)) false)))
  (bind _returnvalue (Default|ChangeUnitInitiative (Variables|Default|GetUnitRef) (Variables|Default|GetBuffCoef) true))
  (Variables|Default|SetIncreasingValue_Initiative _returnvalue)
  (bind _returnvalue_2 (Default|ChangeUnitDamage (Variables|Default|GetUnitRef) (Variables|Default|GetBuffCoef) true))
  (Variables|Default|SetIncreasingValue_Damage _returnvalue_2))

(event EventOnEffectFinished
  (Default|ChangeUnitInitiative (Variables|Default|GetUnitRef) (Math|Conversions|ToFloat(Integer) (* (Variables|Default|GetIncreasingValue_Initiative) -1)) false)
  (Default|ChangeUnitDamage (Variables|Default|GetUnitRef) (Math|Conversions|ToFloat(Integer) (* (Variables|Default|GetIncreasingValue_Damage) -1)) false)
  (|CallParentFunction))

(fn PreparetoRemove
  (|CallParentFunction)
  (Variables|Default|SetBuffCoef 0.0)
  (Variables|Default|SetIncreasingValue_Initiative 0)
  (Variables|Default|SetIncreasingValue_Damage 0)
  (return))