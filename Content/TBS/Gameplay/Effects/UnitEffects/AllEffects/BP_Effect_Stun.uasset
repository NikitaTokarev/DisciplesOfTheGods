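; Stun unit effect that debuffs the affected unit's initiative and accuracy by a percentage set by DebuffCoef.
; On imposition it undoes any earlier reduction, applies the percentage cut and stores the returned deltas, avoiding stacking.
; Finishing reverses the changes, though accuracy restoration uses the stored initiative delta instead of its own.
; PrepareToRemove calls the parent, then zeroes the coefficient and stored values.
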(event EventOnEffectImposed
  (if (== (Variables|Default|GetDecreasingValue_Initiative) 0)
    _
    (else
      (Default|ChangeUnitInitiative (Variables|Default|GetUnitRef) (Math|Conversions|ToFloat(Integer) (* (Variables|Default|GetDecreasingValue_Initiative) -1)) false)))
  (if (== (Variables|Default|GetDecreasingValue_Accuracy) 0)
    _
    (else
      (Default|ChangeUnitAccuracy (Variables|Default|GetUnitRef) (Math|Conversions|ToFloat(Integer) (* (Variables|Default|GetDecreasingValue_Initiative) -1)) false)))
  (bind _returnvalue (Default|ChangeUnitInitiative (Variables|Default|GetUnitRef) (* (Variables|Default|GetDebuffCoef) -1.0) true))
  (Variables|Default|SetDecreasingValue_Initiative _returnvalue)
  (bind _returnvalue_2 (Default|ChangeUnitAccuracy (Variables|Default|GetUnitRef) (* (Variables|Default|GetDebuffCoef) -1.0) true))
  (Variables|Default|SetDecreasingValue_Accuracy _returnvalue_2))

(event EventOnEffectFinished
  (Default|ChangeUnitInitiative (Variables|Default|GetUnitRef) (Math|Conversions|ToFloat(Integer) (* (Variables|Default|GetDecreasingValue_Initiative) -1)) false)
  (Default|ChangeUnitAccuracy (Variables|Default|GetUnitRef) (Math|Conversions|ToFloat(Integer) (* (Variables|Default|GetDecreasingValue_Initiative) -1)) false)
  (|CallParentFunction))

(fn PreparetoRemove
  (|CallParentFunction)
  (Variables|Default|SetDebuffCoef 0.0)
  (Variables|Default|SetDecreasingValue_Initiative 0)
  (Variables|Default|SetDecreasingValue_Accuracy 0)
  (return))