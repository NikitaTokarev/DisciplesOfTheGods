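; BP_Effect_Cleansing is an instant unit effect that cleanses its target unit by removing effects of one type, selected by a boolean flag.
; Execution calls RemoveEffectsByType on UnitRef if that reference is valid, and the damage calculation always returns zero.
; The execution check always passes, leaving an unused branch that would have required the unit to have matching active effects.
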(fn CalculateDamage
  (return 0))

(fn CheckCanbeExecuted
  (return true))

(fn ExecuteInstantEffect
  (bind _unitref (Variables|Default|GetUnitRef)
    (:then
      (Default|RemoveEffectsbyType _unitref true)
      (return))
    (:else
      (return))))