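; Base Blueprint for stackable unit effects in turn-based play, configured from a DT_EFFECTS row.
; Each application appends to parallel Durations and Powers arrays and adds to total EffectPower.
; Updates tick every stack, subtract expired stacks' power, report the longest duration, and finish when none remain.
; The update returns damage, turn permission, sound and text, skipping same-round repeats unless the row allows them.
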(event EventInitializeEffect
  (params (UnitRef :type BP%20Hero%20Base%20Object%20Reference) (Duration :type Integer) (EffectPower :type Float%20%28single-precision%29))
  (Variables|Default|SetUnitRef UnitRef)
  (bind _returnvalue (Utilities|GetDataTableRow "/Game/TBS/Data/Gameplay/DT_EFFECTS.DT_EFFECTS" (Utilities|Struct|BreakDataTableRowHandle (Variables|Default|GetRowHandle)))
    (:then
      (Variables|Default|SetMainData _returnvalue))
    (:RowNotFound
      _))
  (Utilities|Array|Add (Variables|Default|GetDurations) Duration)
  (Utilities|Array|Add (Variables|Default|GetPowers) EffectPower)
  (Variables|Default|SetEffect%20Power (+ EffectPower (Variables|Default|GetEffect%20Power)))
  (Variables|Default|SetEffectData (Utilities|Struct|MakeS_HeroEffect (Variables|Default|GetRowHandle) 0.0 (Variables|Default|GetDuration) (Variables|Default|GetEffect%20Power)))
  (CallFunction|OnEffectImposed))

(fn UpdateEffectState
  (params (Round :type Integer))
  (bind _maindata (Variables|Default|GetMainData))
  (bind (_updatedtext _finishedtext) (Utilities|Struct|BreakS_EffectMain _maindata))
  (if (Utilities|Struct|BreakS_EffectMain (Variables|Default|GetMainData))
    _
    (elif (!= (Variables|Default|GetLastActivatedRound) Round)
      _
      (else
        (LocalVariables|SetL_Response (Utilities|Struct|MakeS_EffectResponse 0 "" true false (CallFunction|CalculateCanUnitTurn)))
        (return (LocalVariables|GetL_Response)))))
  (Variables|Default|SetLastActivatedRound Round)
  (Utilities|Struct|SetmembersinS_EffectResponse (LocalVariables|GetL_Response) (CallFunction|CalculateDamage) (CallFunction|CalculateCanUnitTurn) (Utilities|Struct|BreakS_EffectMain (Variables|Default|GetMainData)))
  (bind _bisfinished (CallFunction|UpdateEffectTimer))
  (bind _output_get (LocalVariables|SetL_Finished _bisfinished))
  (Utilities|Struct|SetmembersinS_EffectResponse (LocalVariables|GetL_Response) (select (LocalVariables|GetL_Finished) _finishedtext _updatedtext) _output_get)
  (Utilities|Struct|SetmembersinS_HeroEffect (Variables|Default|GetEffectData) (CallFunction|GetEffectDuration))
  (if (LocalVariables|GetL_Finished)
    (CallFunction|OnEffectFinished))
  (return (LocalVariables|GetL_Response)))

(fn UpdateEffectTimer
  (for (_array_element _array_index) (Variables|Default|GetDurations)
    (Utilities|Array|SetArrayElem (Variables|Default|GetDurations) _array_index (- _array_element 1))
    (if (== _array_element 0)
      (TBS|Effects|Inherited|OnSubeffectFinished _array_index)))
  (return (== (Utilities|Array|Length (Variables|Default|GetDurations)) 0)))

(fn OnSubeffectFinished
  (params (SubIndex :type Integer))
  (bind _output_get (Variables|Default|SetEffect%20Power (- (Variables|Default|GetEffect%20Power) (Utilities|Array|Get(acopy) (Variables|Default|GetPowers) SubIndex))))
  (Utilities|Struct|SetmembersinS_HeroEffect (Variables|Default|GetEffectData) _output_get)
  (Utilities|Array|RemoveIndex (Variables|Default|GetDurations) SubIndex)
  (Utilities|Array|RemoveIndex (Variables|Default|GetPowers) SubIndex)
  (return))

(fn PreparetoRemove
  (|CallParentFunction)
  (Utilities|Array|Clear (Variables|Default|GetDurations))
  (Utilities|Array|Clear (Variables|Default|GetPowers))
  (return))

(fn GetEffectDuration
  (if (> (Utilities|Array|Length (Variables|Default|GetDurations)) 0)
    (for _array_element (Variables|Default|GetDurations)
      (if (> _array_element (LocalVariables|GetL_MaxDuration))
        (LocalVariables|SetL_MaxDuration _array_element)))
    (return (LocalVariables|GetL_MaxDuration))
    (else
      (return 0))))