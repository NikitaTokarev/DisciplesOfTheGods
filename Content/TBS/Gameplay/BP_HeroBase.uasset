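; Base hero unit for a networked turn-based tactics game, with stats loaded from DT_HeroCharacteristics and gameplay stats built on the authority.
; Server attack, defend and wait actions pass the turn after a delay; attack only announces the target, without applying damage.
; Target selection follows class, reach and position in a six-slot, two-row grid, with column-based priority for melee.
; OnRep handlers and a swappable particle drive HUD feedback and highlights.
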(event Custom|ToggleTurnEffect
  (params (bActivate :type Boolean))
  (bind _returnvalue (Game|GetPlayerController 0))
  (bind _returnvalue_2 (HUD|GetHUD _returnvalue))
  ;[0.2916 0.3826 1 1 32] Highlighting (GUI an Effects)
  (if bActivate
    (Effects|Components|ParticleSystem|SetTemplate (Variables|Default|GetP_TurnHighlighting) "/Game/InfinityBladeEffects/Effects/FX_Mobile/combat/P_Target_Turn.P_Target_Turn")
    (Components|Activation|Activate (Variables|Default|GetP_TurnHighlighting) false)
    (Class|BPIGameHUD|HighlightCurrentCharacter(Message) _returnvalue_2 (Variables|HeroBase|GetPlayerIndex) (Variables|HeroBase|GetPositionInGrid))
    (Class|BPIGameHUD|SetSelectedHeroinPanel(Message) _returnvalue_2 self false)
    (elif (== (Variables|/Script/Engine.ParticleSystemComponent|GetTemplate (Variables|Default|GetP_TurnHighlighting)) "/Game/InfinityBladeEffects/Effects/FX_Mobile/combat/P_Target_Turn.P_Target_Turn")
      (Components|Activation|Deactivate (Variables|Default|GetP_TurnHighlighting))
      (else
        (Class|BPIGameHUD|StopHighlightSelectedHero(Message) (HUD|GetHUD (Game|GetPlayerController 0)) (Variables|HeroBase|GetPlayerIndex) self)))))

(event Custom|ActivateTargetAura
  (params (TargetType :type E_TargetTypes%20Enum :default "NewEnumerator0"))
  (bind _p_turnhighlighting (Variables|Default|GetP_TurnHighlighting))
  ;[0.2916 0.3826 1 1 32] Highlighting (GUI an Effects)
  (bind _returnvalue (Private|GetAuraParticle TargetType))
  (Effects|Components|ParticleSystem|SetTemplate _p_turnhighlighting _returnvalue)
  (Components|Activation|Activate _p_turnhighlighting false))

(event Custom|DeactivateTargetAura
  (bind _p_turnhighlighting (Variables|Default|GetP_TurnHighlighting))
  ;[0.2916 0.3826 1 1 32] Highlighting (GUI an Effects)
  (Components|Activation|Deactivate _p_turnhighlighting)
  (Effects|Components|ParticleSystem|SetTemplate _p_turnhighlighting 0))

(event Custom|AttackTarget_MULTICAST
  (params (AttackedHero :type BP%20Hero%20Base%20Object%20Reference))
  ;[1 0 0.03945 1 32] Attack Execution
  (Development|PrintString (Utilities|String|Append (Utilities|GetDisplayName self) " attacks " (Utilities|GetDisplayName AttackedHero)) true true "(R=1.000000,G=0.000000,B=0.000000,A=1.000000)" 4.0)
  (Class|BPIGroupController|SetAttackedHero(Message) (Game|GetPlayerController 0) AttackedHero 1.0)
  (Networking|SwitchHasAuthority
    (:Authority
      (Utilities|FlowControl|Delay 1.5)
      (Class|BPIGroupController|SwitchTurn(Message) (Game|GetPlayerController 0)))))

(event Custom|AttackTarget_SERVER
  (params (AttackedHero :type BP%20Hero%20Base%20Object%20Reference))
  ;[1 0 0.03945 1 32] Attack Execution
  (CallFunction|AttackTargetMULTICAST AttackedHero))

(event Custom|Defend_SERVER
  ;[0.2837 0.512 1 1 32] Defence
  (Variables|HeroBase|Stats|SetbOnDefence true)
  (Utilities|FlowControl|Delay 1.25)
  (Class|BPIGroupController|SwitchTurn(Message) (Game|GetPlayerController 0)))

(event Custom|OnRoundFinished_Event_0
  (params (NewRound :type Integer))
  ;[1 0.3915 0.6484 1 32] Initializing
  (if (Variables|HeroBase|Stats|GetbIsWaiting)
    (Variables|HeroBase|Stats|SetbIsWaiting false)))

(event Custom|ToggleDefence
  ;[0.2837 0.512 1 1 32] Defence
  (Variables|HeroBase|Stats|SetbOnDefence false))

(event Custom|Waiting_SERVER
  ;[0.5816 1 0.2587 1 32] Waiting
  (Variables|HeroBase|Stats|SetbIsWaiting true)
  (Utilities|FlowControl|Delay 1.25)
  (Class|BPIGroupController|SwitchTurn(Message) (Game|GetPlayerController 0)))

(event EventBeginPlay
  ;[1 0.3915 0.6484 1 32] Initializing
  (bind _returnvalue (Utilities|GetDataTableRow "/Game/TBS/Data/Gameplay/DT_HeroCharacteristics.DT_HeroCharacteristics" (Variables|HeroBase|GetHeroName))
    (:then
      (Variables|HeroBase|Stats|SetAllUnitStats _returnvalue))
    (:RowNotFound
      _))
  (Networking|SwitchHasAuthority
    (:Authority
      (Variables|HeroBase|Stats|SetHeroStats (Utilities|Struct|MakeS_HeroGameplayStats (.Health (Utilities|Struct|BreakS_HeroData (Variables|HeroBase|Stats|GetAllUnitStats))) (.Health (Utilities|Struct|BreakS_HeroData (Variables|HeroBase|Stats|GetAllUnitStats))) (.Armor (Utilities|Struct|BreakS_HeroData (Variables|HeroBase|Stats|GetAllUnitStats))) (.Damage (Utilities|Struct|BreakS_HeroData (Variables|HeroBase|Stats|GetAllUnitStats))) (.Initiative (Utilities|Struct|BreakS_HeroData (Variables|HeroBase|Stats|GetAllUnitStats))) (.Accuracy (Utilities|Struct|BreakS_HeroData (Variables|HeroBase|Stats|GetAllUnitStats))) (.Nimbleness (Utilities|Struct|BreakS_HeroData (Variables|HeroBase|Stats|GetAllUnitStats)))))
      (bind _astbsgame_state (Utilities|Casting|CastToTBSGameState (Game|GetGameState)))
      (bind _output_get (Variables|Default|SetGameState _astbsgame_state))
      (EventDispatchers|AssignOnRoundFinished _output_get (delegate Custom|OnRoundFinished_Event_0)))))

(fn ConstructionScript)

(fn GetAvailableTargets
  (params (Group0 :type Array%20of%20BP%20Hero%20Base%20Object%20References) (Group1 :type Array%20of%20BP%20Hero%20Base%20Object%20References))
  (bind _isinmygroup (Private|IsUnitinMyGroup (TBS|HeroBase|GetPlayerIndex (Utilities|Array|Get(acopy) Group0))))
  (LocalVariables|SetL_MyGroup (select _isinmygroup Group0 Group1))
  (LocalVariables|SetL_EnemyGroup (select _isinmygroup Group1 Group0))
  (LocalVariables|SetL_TargetsAreEnemy (Utilities|Enum|Equal(Enum) (.Class (Utilities|Struct|BreakS_HeroData (Variables|HeroBase|Stats|GetAllUnitStats))) "NewEnumerator0"))
  (switch Utilities|FlowControl|Switch|SwitchonE_TargetAmount (.Targets (Utilities|Struct|BreakS_HeroData (Variables|HeroBase|Stats|GetAllUnitStats)))
    (:NewEnumerator0
      (switch Utilities|FlowControl|Switch|SwitchonE_ReachTypes (.Reach (Utilities|Struct|BreakS_HeroData (Variables|HeroBase|Stats|GetAllUnitStats)))
        (:NewEnumerator0
          (bind _returnvalue (Private|CanUnitAttack (LocalVariables|GetL_MyGroup)))
          (if _returnvalue
            (bind _availabletargets (Private|GetAvailableTargetsforMelee (LocalVariables|GetL_EnemyGroup)))
            (return _availabletargets)
            (else
              (return 0))))
        (:NewEnumerator1
          _)))
    (:NewEnumerator1
      _))
  (return (select (LocalVariables|GetL_TargetsAreEnemy) (LocalVariables|GetL_EnemyGroup) (LocalVariables|GetL_MyGroup))))

(fn GetPlayerIndex
  (return (Variables|HeroBase|GetPlayerIndex)))

(fn GetHeroStats
  (return (Variables|HeroBase|Stats|GetHeroStats)))

(fn GetHeroInitiative
  (return (Utilities|Struct|BreakS_HeroGameplayStats (Variables|HeroBase|Stats|GetHeroStats))))

(fn GetPositioninGrid
  (return (Variables|HeroBase|GetPositionInGrid)))

(fn GetAllUnitStats
  (return (Variables|HeroBase|Stats|GetAllUnitStats)))

(fn GetHeroClass
  (return (.Class (Utilities|Struct|BreakS_HeroData (Variables|HeroBase|Stats|GetAllUnitStats)))))

(fn GetRequiredLeadership
  (return (.Leadership (Utilities|Struct|BreakS_HeroData (Variables|HeroBase|Stats|GetAllUnitStats)))))

(fn GetHeroName
  (return (Variables|HeroBase|GetHeroName)))

(fn GetAvailableTargetsforMelee
  (params (EnemyGroup :type Array%20of%20BP%20Hero%20Base%20Object%20References))
  (for _array_element EnemyGroup
    (Utilities|Array|Add (LocalVariables|GetL_UnitPositions) (TBS|HeroBase|GetPositioninGrid _array_element)))
  (bind _returnvalue (Private|GetUnitColumn))
  (switch int _returnvalue
    (:1
      (bind _returnvalue_2 (Private|TryAddUnitinAvailableTarget (LocalVariables|GetL_UnitPositions) 1 EnemyGroup (LocalVariables|GetL_AvailableTargets)))
      (bind _returnvalue_3 (Private|TryAddUnitinAvailableTarget (LocalVariables|GetL_UnitPositions) 2 EnemyGroup (LocalVariables|GetL_AvailableTargets)))
      (if (or _returnvalue_2 _returnvalue_3)
        (return (LocalVariables|GetL_AvailableTargets))
        (else
          (bind _returnvalue_4 (Private|TryAddUnitinAvailableTarget (LocalVariables|GetL_UnitPositions) 3 EnemyGroup (LocalVariables|GetL_AvailableTargets)))
          (if _returnvalue_4
            (return (LocalVariables|GetL_AvailableTargets))
            (else
              (bind _returnvalue_5 (Private|TryAddUnitinAvailableTarget (LocalVariables|GetL_UnitPositions) 4 EnemyGroup (LocalVariables|GetL_AvailableTargets)))
              (bind _returnvalue_6 (Private|TryAddUnitinAvailableTarget (LocalVariables|GetL_UnitPositions) 5 EnemyGroup (LocalVariables|GetL_AvailableTargets)))
              (if (or _returnvalue_5 _returnvalue_6)
                (return (LocalVariables|GetL_AvailableTargets))
                (else
                  (return (Utilities|Array|MakeArray (Utilities|Array|Get(acopy) EnemyGroup (Utilities|Array|FindItem (LocalVariables|GetL_UnitPositions) 6)))))))))))
    (:2
      (bind _returnvalue_7 (Private|TryAddUnitinAvailableTarget (LocalVariables|GetL_UnitPositions) 1 EnemyGroup (LocalVariables|GetL_AvailableTargets)))
      (bind _returnvalue_8 (Private|TryAddUnitinAvailableTarget (LocalVariables|GetL_UnitPositions) 2 EnemyGroup (LocalVariables|GetL_AvailableTargets)))
      (bind _returnvalue_9 (Private|TryAddUnitinAvailableTarget (LocalVariables|GetL_UnitPositions) 3 EnemyGroup (LocalVariables|GetL_AvailableTargets)))
      (if (Math|Boolean|ORBoolean _returnvalue_7 _returnvalue_8 _returnvalue_9)
        (return (LocalVariables|GetL_AvailableTargets))
        (else
          (Private|TryAddUnitinAvailableTarget (LocalVariables|GetL_UnitPositions) 4 EnemyGroup (LocalVariables|GetL_AvailableTargets))
          (Private|TryAddUnitinAvailableTarget (LocalVariables|GetL_UnitPositions) 5 EnemyGroup (LocalVariables|GetL_AvailableTargets))
          (Private|TryAddUnitinAvailableTarget (LocalVariables|GetL_UnitPositions) 6 EnemyGroup (LocalVariables|GetL_AvailableTargets))
          (return (LocalVariables|GetL_AvailableTargets)))))
    (:3
      (bind _returnvalue_10 (Private|TryAddUnitinAvailableTarget (LocalVariables|GetL_UnitPositions) 3 EnemyGroup (LocalVariables|GetL_AvailableTargets)))
      (bind _returnvalue_11 (Private|TryAddUnitinAvailableTarget (LocalVariables|GetL_UnitPositions) 2 EnemyGroup (LocalVariables|GetL_AvailableTargets)))
      (if (or _returnvalue_10 _returnvalue_11)
        (return (LocalVariables|GetL_AvailableTargets))
        (else
          (bind _returnvalue_12 (Private|TryAddUnitinAvailableTarget (LocalVariables|GetL_UnitPositions) 1 EnemyGroup (LocalVariables|GetL_AvailableTargets)))
          (if _returnvalue_12
            (return (LocalVariables|GetL_AvailableTargets))
            (else
              (bind _returnvalue_13 (Private|TryAddUnitinAvailableTarget (LocalVariables|GetL_UnitPositions) 6 EnemyGroup (LocalVariables|GetL_AvailableTargets)))
              (bind _returnvalue_14 (Private|TryAddUnitinAvailableTarget (LocalVariables|GetL_UnitPositions) 5 EnemyGroup (LocalVariables|GetL_AvailableTargets)))
              (if (or _returnvalue_13 _returnvalue_14)
                (return (LocalVariables|GetL_AvailableTargets))
                (else
                  (return (Utilities|Array|MakeArray (Utilities|Array|Get(acopy) EnemyGroup (Utilities|Array|FindItem (LocalVariables|GetL_UnitPositions) 4)))))))))))))

(fn GetAuraParticle
  (params (TargetType :type E_TargetTypes%20Enum :default "NewEnumerator0"))
  (return (Utilities|Select :Index TargetType :NewEnumerator0 0 :NewEnumerator1 "/Game/InfinityBladeEffects/Effects/FX_Mobile/combat/P_Target_Attack.P_Target_Attack" :NewEnumerator2 "/Game/InfinityBladeEffects/Effects/FX_Mobile/combat/P_Target_Healing.P_Target_Healing" :NewEnumerator3 "/Game/InfinityBladeEffects/Effects/FX_Mobile/combat/P_Target_Buff.P_Target_Buff")))

(fn GetTargetAmount
  (return (.Targets (Utilities|Struct|BreakS_HeroData (Variables|HeroBase|Stats|GetAllUnitStats)))))

(fn IsUnitinMyGroup
  (params (GroupIndex :type Integer))
  (return (== GroupIndex (Variables|HeroBase|GetPlayerIndex))))

(fn GetUnitRow
  (return (select (< (Variables|HeroBase|GetPositionInGrid) 4) 1 2)))

(fn CanUnitAttack
  (params (MyGroup :type Array%20of%20BP%20Hero%20Base%20Object%20References))
  (if (== (Private|GetUnitRow) 2)
    (Utilities|Array|ForEachLoopwithBreak MyGroup :!label _label
      (:LoopBody
        (if (not (!= (TBS|HeroBase|GetPositioninGrid) 1))
          (LocalVariables|SetL_CanAttack false)
          (goto _label Break)))
      (:Completed
        (return (LocalVariables|GetL_CanAttack))))
    (else
      (return true))))

(fn GetUnitColumn
  (return (select (or (== (Variables|HeroBase|GetPositionInGrid) 1) (== (Variables|HeroBase|GetPositionInGrid) 4)) 1 (select (or (== (Variables|HeroBase|GetPositionInGrid) 2) (== (Variables|HeroBase|GetPositionInGrid) 5)) 2 3))))

(fn TryAddUnitinAvailableTarget
  (params (Positions :type Array%20of%20Integers) (RequiredPosition :type Integer) (TargetUnits :type Array%20of%20BP%20Hero%20Base%20Object%20References) (ArrayToAdd :type Array%20of%20BP%20Hero%20Base%20Object%20References))
  (bind _output_get (LocalVariables|SetL_Index (Utilities|Array|FindItem Positions RequiredPosition)))
  (if (!= _output_get -1)
    (bind _returnvalue (Utilities|Array|Add ArrayToAdd (Utilities|Array|Get(acopy) TargetUnits (LocalVariables|GetL_Index))))
    (return (!= _returnvalue -1))
    (else
      (return false))))

(fn GetUnitHealth
  (return (Utilities|Struct|BreakS_HeroGameplayStats (Variables|HeroBase|Stats|GetHeroStats)) (Utilities|Struct|BreakS_HeroData (Variables|HeroBase|Stats|GetAllUnitStats))))

(fn GetUnitIcon
  (return (Utilities|Struct|BreakS_HeroData (Variables|HeroBase|Stats|GetAllUnitStats))))

(fn GetUnitDefaultHealth
  (return (Utilities|Struct|BreakS_HeroData (Variables|HeroBase|Stats|GetAllUnitStats))))

(fn GetHeroDisplayName
  (return (Utilities|Struct|BreakS_HeroData (Variables|HeroBase|Stats|GetAllUnitStats))))

(fn GetUnitSelectedIcon
  (return (Utilities|Struct|BreakS_HeroData (Variables|HeroBase|Stats|GetAllUnitStats))))

(fn OnRepBonDefence
  (Class|BPIGameHUD|StopHighlightingTurningHero(Message) (HUD|GetHUD (Game|GetPlayerController 0)))
  (Class|BPIGameHUD|ToggleDefenceEffect(Message) (HUD|GetHUD (Game|GetPlayerController 0)) self (Variables|HeroBase|Stats|GetbOnDefence))
  (return))

(fn GetonDefence
  (return (Variables|HeroBase|Stats|GetbOnDefence)))

(fn OnRepBIsWaiting
  (Class|BPIPlayerGroupController|UpdateWaitingButton(Message) (Game|GetPlayerController 0) (Variables|HeroBase|Stats|GetbIsWaiting))
  (if (Variables|HeroBase|Stats|GetbIsWaiting)
    (Class|BPIGameHUD|StopHighlightingTurningHero(Message) (HUD|GetHUD (Game|GetPlayerController 0)))
    (Class|BPIGameHUD|PlayWaitingEffect(Message) (HUD|GetHUD (Game|GetPlayerController 0)) self)
    (Networking|SwitchHasAuthority
      (:Authority
        (Default|ControlUnitWaiting (Variables|Default|GetGameState) self)
        (return))
      (:Remote
        (return)))
    (else
      (return))))

(fn GetIsWaiting
  (return (Variables|HeroBase|Stats|GetbIsWaiting)))