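; Base class for turn-based unit abilities, loading its settings from a DT_ABILITIES row when initialized with an owner unit.
; Using it records the round, starts the cooldown and builds per-target attack results from hit/crit checks, damage and chance-rolled effects.
; UpdateAbilityState ticks cooldowns and checks reuse limits, with CanUseAbilityNow as an always-true default hook.
; Critical hits multiply damage by 1.75; results are returned rather than applied to targets.
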(event Custom|InitializeAbility
  (params (OwnerUnit :type BP%20Hero%20Base%20Object%20Reference))
  (Variables|Default|SetOwnerUnit OwnerUnit)
  (bind _returnvalue (Utilities|GetDataTableRow "/Game/TBS/Data/Gameplay/DT_ABILITIES.DT_ABILITIES" (Utilities|Struct|BreakDataTableRowHandle (Variables|Default|GetAbilityRow)))
    (:then
      (Variables|Default|SetAbilityData _returnvalue))))

(fn UseUnitAbility
  (params (Targets :type Array%20of%20BP%20Hero%20Base%20Object%20References) (Round :type Integer))
  (Variables|Default|SetLastUsingRound Round)
  (Variables|Default|SetbAbilityHasBeenAlreadyUsed true)
  (Variables|Default|SetCooldown (.Cooldown (Utilities|Struct|BreakS_AbilityData (Variables|Default|GetAbilityData))))
  (bind (_returnvalue _maxeffectcount) (TBS|Ability|Inherited|ExecuteAbility Targets))
  (return _returnvalue _maxeffectcount))

(fn FinishTurnAfterAbility
  (return (.bFinishingTurn (Utilities|Struct|BreakS_AbilityData (Variables|Default|GetAbilityData)))))

(fn UpdateAbilityState
  (params (RoundNumber :type Integer))
  (if (not (.bOneTimeUse (Utilities|Struct|BreakS_AbilityData (Variables|Default|GetAbilityData))))
    (if (!= RoundNumber (Variables|Default|GetLastUsingRound))
      _
      (elif (.bCanUseSeveralTimesPerRound (Utilities|Struct|BreakS_AbilityData (Variables|Default|GetAbilityData)))
        _
        (else
          (return false))))
    (if (== (Variables|Default|GetCooldown) 0)
      _
      (else
        (bind _result (Math|Integer|DecrementInt (Variables|Default|GetCooldown))
          (:%20%20
            (if (== _result 0)
              _
              (else
                (return false)))))))
    (if (TBS|Ability|Inherited|CanUseAbilityNow RoundNumber)
      (return true)
      (else
        (return false)))
    (else
      (return (Variables|Default|GetbAbilityHasBeenAlreadyUsed)))))

(fn CanUseAbilityNow
  (params (RoundNumber :type Integer))
  (return true))

(fn GetTargetsAreEnemy
  (return (.bTargetsAreEnemy (Utilities|Struct|BreakS_AbilityData (Variables|Default|GetAbilityData)))))

(fn GetNumberOfTargets
  (return (.Target (Utilities|Struct|BreakS_AbilityData (Variables|Default|GetAbilityData)))))

(fn GetAbilityReach
  (return (.ReachTypes (Utilities|Struct|BreakS_AbilityData (Variables|Default|GetAbilityData)))))

(fn GetAbilityData
  (return (Variables|Default|GetAbilityData)))

(fn ExecuteAbility
  (params (AbilityTargets :type Array%20of%20BP%20Hero%20Base%20Object%20References))
  (for _array_element AbilityTargets
    (bind (_issuccessful _iscritical) (TBS|Ability|Inherited|CalculateIsUsingSuccessful _array_element))
    (if _issuccessful
      (bind (_source _damage) (TBS|Ability|Inherited|CalculateDamage _array_element _iscritical))
      (bind _returnvalue (TBS|Ability|Inherited|CalculateEffects _array_element))
      (Utilities|Array|Add (LocalVariables|GetL_Results) (Utilities|Struct|MakeS_AttackResult _array_element _issuccessful (TBS|Ability|Inherited|ShouldCalculateDamage) _source _damage _returnvalue _iscritical))
      (if (> (Utilities|Array|Length _returnvalue) (LocalVariables|GetL_MaxEffectCount))
        (LocalVariables|SetL_MaxEffectCount (Utilities|Array|Length _returnvalue)))
      (else
        (Utilities|Array|Add (LocalVariables|GetL_Results) (Utilities|Struct|MakeS_AttackResult _array_element false false)))))
  (return (LocalVariables|GetL_Results) (LocalVariables|GetL_MaxEffectCount)))

(fn CalculateIsUsingSuccessful
  (params (AttackedUnit :type BP%20Hero%20Base%20Object%20Reference))
  (bind _abilitydata (Variables|Default|GetAbilityData))
  (bind (_bcanabilitymisses _bhascriticalhit) (Utilities|Struct|BreakS_AbilityData _abilitydata))
  (if _bcanabilitymisses
    (bind (_ishit _iscritical) (Default|CalculateHitorMiss (Variables|Default|GetOwnerUnit) AttackedUnit))
    (return _ishit (select _bhascriticalhit _iscritical false))
    (else
      (return true false))))

(fn CalculateDamage
  (params (AttackedUnit :type BP%20Hero%20Base%20Object%20Reference) (IsCritical :type Boolean))
  (bind _abilitydata (Variables|Default|GetAbilityData))
  (bind (_source _damage) (Utilities|Struct|BreakS_AbilityData _abilitydata))
  (if IsCritical
    (for _array_element (.Damage (Utilities|Struct|BreakS_AbilityData (Variables|Default|GetAbilityData)))
      (Utilities|Array|Add (LocalVariables|GetL_Damage) (Math|Float|Round (* _array_element 1.75))))
    (return (.Source (Utilities|Struct|BreakS_AbilityData (Variables|Default|GetAbilityData))) (LocalVariables|GetL_Damage))
    (else
      (return _source _damage))))

(fn CalculateEffects
  (params (TargetUnit :type BP%20Hero%20Base%20Object%20Reference))
  (bind _abilitydata (Variables|Default|GetAbilityData))
  (bind _effects (Utilities|Struct|BreakS_AbilityData _abilitydata))
  (if (!= (Utilities|Array|Length _effects) 0)
    (for _array_element _effects
      (if (Math|Random|RandomBoolwithWeight (.EffectChance (Utilities|Struct|BreakS_HeroEffect _array_element)))
        (Utilities|Array|Add (LocalVariables|GetL_Effects) _array_element)))
    (return (LocalVariables|GetL_Effects))
    (else
      (return 0))))

(fn ShouldCalculateDamage
  (return (.bCalculateDamage (Utilities|Struct|BreakS_AbilityData (Variables|Default|GetAbilityData)))))

(fn GetAbilityDamageSources
  (return (.Source (Utilities|Struct|BreakS_AbilityData (Variables|Default|GetAbilityData)))))