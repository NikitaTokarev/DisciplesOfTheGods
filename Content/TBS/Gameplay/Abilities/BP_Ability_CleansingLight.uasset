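; Cleansing Light ability for the turn-based game, which applies fixed negative damage (in effect a heal) and a single effect to each target.
; ExecuteAbility builds an always-successful attack result per target from CalculateDamage and CalculateEffects, returning the results with the highest effect count.
; The effect comes from the first EffectRows entry, with guaranteed chance and zero duration.
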(fn ExecuteAbility
  (params (AbilityTargets :type Array%20of%20BP%20Hero%20Base%20Object%20References))
  (for _array_element AbilityTargets
    (bind (_source _damage) (CallFunction|CalculateDamage _array_element))
    (bind _returnvalue (CallFunction|CalculateEffects _array_element))
    (Utilities|Array|Add (LocalVariables|GetL_Results) (Utilities|Struct|MakeS_AttackResult _array_element true true _source _damage _returnvalue))
    (if (> (Utilities|Array|Length _returnvalue) (LocalVariables|GetL_MaxEffectCount))
      (LocalVariables|SetL_MaxEffectCount (Utilities|Array|Length _returnvalue))))
  (return (LocalVariables|GetL_Results) (LocalVariables|GetL_MaxEffectCount)))

(fn CalculateDamage
  (params (AttackedUnit :type BP%20Hero%20Base%20Object%20Reference))
  (return (Utilities|Array|MakeArray "NewEnumerator4") (Utilities|Array|MakeArray -45)))

(fn CalculateEffects
  (params (TargetUnit :type BP%20Hero%20Base%20Object%20Reference))
  (return (Utilities|Array|MakeArray (Utilities|Struct|MakeS_HeroEffect (Utilities|Array|Get(acopy) (Variables|Default|GetEffectRows)) 1.0 0 0.0))))