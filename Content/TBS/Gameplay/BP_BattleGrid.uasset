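; BP_BattleGrid is a six-cell battle grid, tagged with a player index, that places a hero group in TBS battles.
; On BeginPlay the server registers it with TBSGameMode.
; ControlOfGroupSpawning spawns each hero at its cell component's transform, owned by the supplied controller, then reports it to that controller.
; GetTruePositionInGrid mirrors the two halves of the grid for player 0, but spawning does not use it.
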(event Custom|ControlOfGroupSpawning
  (params (Group :type Array%20of%20S%20Battle%20Group%20Structures) (PlayerIndex :type Integer) (Controller :type Controller%20Object%20Reference))
  (for _array_element Group
    (bind _returnvalue (Game|SpawnActorfromClass (.HeroClass (Utilities|Struct|BreakS_BattleGroup _array_element)) (Math|Transform|MakeTransform (.CellLocation (CallFunction|GetCellLocationandRotation (.CellIndex (Utilities|Struct|BreakS_BattleGroup _array_element)))) (.CellRotation (CallFunction|GetCellLocationandRotation (.CellIndex (Utilities|Struct|BreakS_BattleGroup _array_element)))) "1,1,1") "AlwaysSpawn" Controller PlayerIndex (.CellIndex (Utilities|Struct|BreakS_BattleGroup _array_element)) (Pawn|GetControlledPawn Controller)))
    (Class|BPIGroupController|AddUnitinGroup(Message) Controller _returnvalue)))

(event EventBeginPlay
  (Networking|SwitchHasAuthority
    (:Authority
      (bind _astbsgame_mode (Utilities|Casting|CastToTBSGameMode (Game|GetGameMode)))
      (Default|AddBattleGrid _astbsgame_mode self))))

(fn ConstructionScript)

(fn GetPlayerIndex
  (return (Variables|Default|GetPlayerIndex)))

(fn GetCellLocationandRotation
  (params (CellIndex :type Integer))
  (bind _cell1 (Variables|Default|GetCell1))
  (bind _cell2 (Variables|Default|GetCell2))
  (bind _cell3 (Variables|Default|GetCell3))
  (bind _cell4 (Variables|Default|GetCell4))
  (bind _cell5 (Variables|Default|GetCell5))
  (bind _cell6 (Variables|Default|GetCell6))
  (bind _arrow (Variables|Default|GetArrow))
  (bind _returnvalue (Utilities|Select :Index CellIndex :Option%200 _arrow :Option%201 _cell1 :Option%202 _cell2 :Option%203 _cell3 :Option%204 _cell4 :Option%205 _cell5 :Option%206 _cell6))
  (return (Transformation|GetWorldLocation _returnvalue) (Transformation|GetWorldRotation _returnvalue)))

(fn GetTruePositioninGrid
  (params (Position :type Integer))
  (if (== (Variables|Default|GetPlayerIndex) 0)
    (switch int Position
      (:1
        (return 4))
      (:2
        (return 5))
      (:3
        (return 6))
      (:4
        (return 1))
      (:5
        (return 2))
      (:6
        (return 3)))
    (else
      (return Position))))