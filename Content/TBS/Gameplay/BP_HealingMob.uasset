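; BP_HealingMob is a turn-based unit Blueprint that, by its name, acts as a healer mob.
; It overrides hit resolution to always land without critical hits and takes its damage value straight from the unit's Damage stat.
; PlayAttackEffects loops over the attack results and spawns an ice aura particle below each affected unit's origin.
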(event EventBeginPlay
  (|CallParentFunction) ; This node is disabled and will not be called.\nDrag off pins to build functionality.
)

(event EventPlayAttackEffects
  (bind _returnvalue (CallFunction|GetAttackResults))
  (for _array_element _returnvalue
    (Effects|SpawnEmitteratLocation "/Game/InfinityBladeEffects/Effects/FX_Skill_Aura/P_Aura_Ice_Ending_01.P_Aura_Ice_Ending_01" (- (Transformation|GetActorLocation (Utilities|Struct|BreakS_AttackResult _array_element)) "0, 0,125.000000"))))

(fn ConstructionScript
  (|CallParentFunction))

(fn CalculateHitorMiss
  (params (AttackedHero :type BP%20Hero%20Base%20Object%20Reference))
  (return true false))

(fn CalculateDamage
  (return (.Damage (Utilities|Struct|BreakS_HeroGameplayStats (CallFunction|GetUnitStats)))))