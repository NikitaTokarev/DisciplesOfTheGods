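; BP_Hero_Rage is the Rage hero character Blueprint for the turn-based gameplay, built on a parent class that supplies its behavior.
; PlayVisualEffects activates the PHellBlade effect with a reset when an ability is being used, and has no branch to switch it off.
; The server turn toggle and construction script only forward to the parent, while BeginPlay and overlap events are disabled stubs.
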(event EventBeginPlay
  (|CallParentFunction) ; This node is disabled and will not be called.\nDrag off pins to build functionality.
)

(event Collision|EventActorBeginOverlap
  (params (OtherActor :type Actor%20Object%20Reference))
  (|CallParentFunction OtherActor) ; This node is disabled and will not be called.\nDrag off pins to build functionality.
)

(event EventPlayVisualEffects
  (params (bIsAbilityUsing :type Boolean) (AttackIndex :type Integer))
  (if bIsAbilityUsing
    (Components|Activation|Activate (Variables|Default|GetP_HellBlade) true)))

(event EventToggleUnitTurnSERVER
  (params (bActivate :type Boolean))
  (|CallParentFunction bActivate))

(fn ConstructionScript
  (|CallParentFunction))