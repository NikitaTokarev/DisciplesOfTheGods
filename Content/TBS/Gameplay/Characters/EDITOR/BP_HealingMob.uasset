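; BP_HealingMob is a turn-based unit that, judging by its name and particles, heals its targets.
; It overrides combat calculations to always hit, never crit and use the Damage stat directly.
; It applies its stat effects only when the target already has active effects of a given type.
; Visuals move pre-placed particles onto targets: one for the ability's first target, or one of six per regular attack result.
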(event EventBeginPlay
  (|CallParentFunction)
  (Variables|Default|SetAttackParticles (Utilities|Array|MakeArray (Variables|Default|GetP_HealingParticle_1) (Variables|Default|GetP_HealingParticle_2) (Variables|Default|GetP_HealingParticle_3) (Variables|Default|GetP_HealingParticle_4) (Variables|Default|GetP_HealingParticle_5) (Variables|Default|GetP_HealingParticle_6))))

(event EventPlayVisualEffects
  (params (bIsAbilityUsing :type Boolean) (AttackIndex :type Integer))
  (if bIsAbilityUsing
    (bind _returnvalue (CallFunction|GetAttackResults))
    (Transformation|SetWorldLocation (Variables|Default|GetP_AbilityParticle) (Transformation|GetActorLocation (Utilities|Struct|BreakS_AttackResult (Utilities|Array|Get(acopy) _returnvalue))) false false)
    (Components|Activation|Activate (Variables|Default|GetP_AbilityParticle) true)
    (else
      (bind _returnvalue_2 (CallFunction|GetAttackResults))
      (for (_array_element _array_index) _returnvalue_2
        (Transformation|SetWorldLocation (Utilities|Array|Get(acopy) (Variables|Default|GetAttackParticles) _array_index) (- (Transformation|GetActorLocation (Utilities|Struct|BreakS_AttackResult _array_element)) "0, 0,125.000000") false false)
        (Components|Activation|Activate (Utilities|Array|Get(acopy) (Variables|Default|GetAttackParticles) _array_index) true)))))

(fn ConstructionScript
  (|CallParentFunction))

(fn CalculateHitorMiss
  (params (AttackedHero :type BP%20Hero%20Base%20Object%20Reference))
  (return true false))

(fn CalculateDamage
  (params (AttackedUnit :type BP%20Hero%20Base%20Object%20Reference) (bIsCritical :type Boolean))
  (return (Utilities|Struct|BreakS_HeroGameplayStats (CallFunction|GetUnitStats))))

(fn CalculateEffects
  (params (AttackedUnit :type BP%20Hero%20Base%20Object%20Reference))
  (bind _returnvalue (Default|HasUnitActiveEffectsbyType AttackedUnit true))
  (if _returnvalue
    (return (Utilities|Struct|BreakS_HeroGameplayStats (CallFunction|GetUnitStats)))
    (else
      (return 0))))