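; BP_MagicMob is a turn-based magic enemy character that shows attack particles beneath every unit it hits.
; BeginPlay gathers six particle components into an array that serves as a fixed pool.
; PlayVisualEffects loops over the attack results, moves the particle at the matching index to just below each attacked unit, and activates it.
; The index is not bounds-checked, so only six simultaneous targets are covered.
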(event EventBeginPlay
  (|CallParentFunction)
  (Variables|Default|SetAttackParticles (Utilities|Array|MakeArray (Variables|Default|GetP_AttackParticle_01) (Variables|Default|GetP_AttackParticle_02) (Variables|Default|GetP_AttackParticle_03) (Variables|Default|GetP_AttackParticle_04) (Variables|Default|GetP_AttackParticle_05) (Variables|Default|GetP_AttackParticle_06))))

(event EventPlayVisualEffects
  (params (bIsAbilityUsing :type Boolean) (AttackIndex :type Integer))
  (bind _returnvalue (CallFunction|GetAttackResults))
  (for (_array_element _array_index) _returnvalue
    (Transformation|SetWorldLocation (Utilities|Array|Get(acopy) (Variables|Default|GetAttackParticles) _array_index) (- (Transformation|GetActorLocation (Utilities|Struct|BreakS_AttackResult _array_element)) "0, 0,140.000000") false false)
    (Components|Activation|Activate (Utilities|Array|Get(acopy) (Variables|Default|GetAttackParticles) _array_index) true)))

(fn ConstructionScript
  (|CallParentFunction))