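; Empire Titan character Blueprint for the TBS game, adding a weapon-style trail effect and an assassin positioning point to its parent class.
; On BeginPlay it creates a dynamic material for the trail particle component and sets its opacity.
; PlayTrailEffects runs an anim trail between two sockets for a short fixed delay.
; GetPositionForAssassin returns a point a fixed distance behind the Titan, keeping its height.
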(event EventBeginPlay
  (bind _p_animtraileffect (Variables|Default|GetP_AnimTrailEffect))
  (|CallParentFunction)
  (bind _returnvalue (Rendering|Material|CreateDynamicMaterialInstance _p_animtraileffect 0 (Rendering|Material|GetMaterial _p_animtraileffect 0) "None" :!class /Script/Engine.PrimitiveComponent))
  (bind _output_get (Variables|Default|SetMI_TrailEffect _returnvalue))
  (Rendering|Material|SetScalarParameterValue _output_get "Opacity" 4.0 :!class /Script/Engine.MaterialInstanceDynamic))

(event EventPlayTrailEffects
  (params (AttackType :type Integer))
  (Effects|Particles|Trails|BeginTrails (Variables|Default|GetP_AnimTrailEffect) "S_Trail_01" "S_Trail_02" "ETrailWidthMode_FromCentre" 1.5)
  (Utilities|FlowControl|Delay 0.6)
  (Effects|Particles|Trails|EndTrails (Variables|Default|GetP_AnimTrailEffect)))

(fn ConstructionScript)

(fn GetPositionforAssassin
  (bind _returnvalue (Transformation|GetActorForwardVector))
  (bind _returnvalue_2 (* _returnvalue 275.0))
  (return (- (Transformation|GetActorLocation) (Math|Vector|MakeVector (.x _returnvalue_2) (.y _returnvalue_2) 0.0))))