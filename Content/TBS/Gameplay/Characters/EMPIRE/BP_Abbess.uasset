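; BP_Abbess is the Empire Abbess unit Blueprint for the turn-based game, apparently a healer given its healing particle effect.
; It overrides the combat calculations to always hit, never crit and use the unit's Damage stat unmodified.
; The unit's Effects are returned only when the target already has active effects of the queried type.
; Its visual event activates either the ability or the healing particle system.
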(event EventPlayVisualEffects
  (params (bIsAbilityUsing :type Boolean) (AttackIndex :type Integer))
  (if bIsAbilityUsing
    (Components|Activation|Activate (Variables|Default|GetP_AbilityEffect) true)
    (else
      (Components|Activation|Activate (Variables|Default|GetP_HealingEffect) true))))

(event EventBeginPlay
  (|CallParentFunction))

(fn ConstructionScript)

(fn CalculateHitorMiss
  (params (AttackedHero :type BP%20Hero%20Base%20Object%20Reference))
  (return true false))

(fn CalculateDamage
  (params (AttackedUnit :type BP%20Hero%20Base%20Object%20Reference) (bIsCritical :type Boolean))
  (return (Utilities|Struct|BreakS_HeroGameplayStats (CallFunction|GetUnitStats))))

(fn CalculateEffects
  (params (AttackedUnit :type BP%20Hero%20Base%20Object%20Reference))
  (bind _returnvalue (Default|HasUnitActiveEffectsbyType AttackedUnit true))
  (if _returnvalue
    (return (Utilities|Struct|BreakS_HeroGameplayStats (CallFunction|GetUnitStats)))
    (else
      (return 0))))