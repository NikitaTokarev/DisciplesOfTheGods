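; Assassin unit Blueprint for the Empire faction, with a teleporting backstab attack visual.
; PlayVisualEffects moves it behind the first attacked unit via GetPositionForAssassin, turned 180° from its start yaw, then returns it to the transform cached at BeginPlay.
; Smoke and beam particles, mesh visibility toggles and fixed delays sequence the teleport.
; PlayTrailEffects briefly runs a socket-based trail tinted through a dynamic material instance.
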(event EventBeginPlay
  (bind _p_animtraileffect (Variables|Default|GetP_AnimTrailEffect))
  (|CallParentFunction)
  (Variables|Default|SetOriginalTransform (Transformation|GetActorTransform))
  (bind _returnvalue (Rendering|Material|CreateDynamicMaterialInstance _p_animtraileffect 0 (Rendering|Material|GetMaterial _p_animtraileffect 0) "None" :!class /Script/Engine.PrimitiveComponent))
  (bind _output_get (Variables|Default|SetMI_TrailEffect _returnvalue))
  (Rendering|Material|SetScalarParameterValue _output_get "Opacity" 4.0 :!class /Script/Engine.MaterialInstanceDynamic)
  (Rendering|Material|SetVectorParameterValue _output_get "Color" "(R=0.116580,G=0.004881,B=0.575000,A=1.000000)" :!class /Script/Engine.MaterialInstanceDynamic)
  (Transformation|DetachFromComponent (Variables|Default|GetP_AuraHighlighting) "KeepWorld" "KeepWorld" "KeepWorld" true))

(event EventPlayVisualEffects
  (params (bIsAbilityUsing :type Boolean) (AttackIndex :type Integer))
  (bind _originaltransform (Variables|Default|GetOriginalTransform))
  (bind _originaltransform_2 (Variables|Default|GetOriginalTransform))
  (bind _rotation (Math|Transform|BreakTransform _originaltransform))
  (Components|Activation|Activate (Variables|Default|GetP_TeleportEffect_Smoke) true)
  (Utilities|FlowControl|Delay 0.075)
  (bind _returnvalue (CallFunction|GetAttackResults))
  (Transformation|SetActorLocationAndRotation (CallFunction|GetPositionforAssassin (Utilities|Struct|BreakS_AttackResult (Utilities|Array|Get(acopy) _returnvalue))) (Math|Rotator|MakeRotator (.roll _rotation) (.pitch _rotation) (+ (.yaw _rotation) 1.8e+02)))
  (Components|Activation|Activate (Variables|Default|GetP_TeleportEffect_Beam) true)
  (Utilities|FlowControl|Delay 0.15)
  (Development|SetHiddeninGame (Variables|Default|GetSkeletalMesh) false true)
  (Utilities|FlowControl|Delay 1.6)
  (Transformation|SetRelativeLocation (Variables|Default|GetP_TeleportEffect_Smoke) "0,6.000000,-95.000000" false false)
  (Components|Activation|Activate (Variables|Default|GetP_TeleportEffect_Smoke) true)
  (Development|SetHiddeninGame (Variables|Default|GetSkeletalMesh) true true)
  (Utilities|FlowControl|Delay 0.875)
  (Transformation|SetRelativeLocation (Variables|Default|GetP_TeleportEffect_Smoke) "-99.000000,6.000000,-95.000000" false false)
  (Transformation|SetActorLocationAndRotation (.location _originaltransform_2) (.rotation _originaltransform_2))
  (Components|Activation|Activate (Variables|Default|GetP_TeleportEffect_Smoke) true)
  (Development|SetHiddeninGame (Variables|Default|GetSkeletalMesh) false true))

(event EventPlayTrailEffects
  (params (AttackType :type Integer))
  (Effects|Particles|Trails|BeginTrails (Variables|Default|GetP_AnimTrailEffect) "S_Trail_01" "S_Trail_02" "ETrailWidthMode_FromCentre" 1.5)
  (Utilities|FlowControl|Delay 0.4)
  (Effects|Particles|Trails|EndTrails (Variables|Default|GetP_AnimTrailEffect)))

(fn ConstructionScript)

(fn GetPositionforAssassin
  (bind _returnvalue (Transformation|GetActorForwardVector))
  (bind _returnvalue_2 (* _returnvalue 2.7e+02))
  (return (- (Transformation|GetActorLocation) (Math|Vector|MakeVector (.x _returnvalue_2) (.y _returnvalue_2) 0.0))))