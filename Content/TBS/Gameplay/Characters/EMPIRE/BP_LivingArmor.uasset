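; BP_LivingArmor is the Living Armor character Blueprint in the Empire faction, adding a weapon-style trail effect to the parent character's behavior.
; On BeginPlay it creates a dynamic material for its anim trail particle component and sets the opacity and a blue color.
; The PlayTrailEffects event begins trails between two trail sockets, then ends them after a one-second delay.
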(event EventBeginPlay
  (bind _p_animtraileffect (Variables|Default|GetP_AnimTrailEffect))
  (|CallParentFunction)
  (bind _returnvalue (Rendering|Material|CreateDynamicMaterialInstance _p_animtraileffect 0 (Rendering|Material|GetMaterial _p_animtraileffect 0) "None" :!class /Script/Engine.PrimitiveComponent))
  (bind _output_get (Variables|Default|SetMI_TrailEffect _returnvalue))
  (Rendering|Material|SetScalarParameterValue _output_get "Opacity" 1e+01 :!class /Script/Engine.MaterialInstanceDynamic)
  (Rendering|Material|SetVectorParameterValue _output_get "Color" "(R=0.092998,G=0.195662,B=0.834375,A=1.000000)" :!class /Script/Engine.MaterialInstanceDynamic))

(event EventPlayTrailEffects
  (params (AttackType :type Integer))
  (Effects|Particles|Trails|BeginTrails (Variables|Default|GetP_AnimTrailEffect) "S_Trail_01" "S_Trail_02" "ETrailWidthMode_FromCentre" 1.5)
  (Utilities|FlowControl|Delay 1.0)
  (Effects|Particles|Trails|EndTrails (Variables|Default|GetP_AnimTrailEffect)))

(fn ConstructionScript)