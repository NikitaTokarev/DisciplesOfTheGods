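; Empire Holy Archer unit Blueprint that adds an impact particle effect and a glowing appear/disappear effect for its gear.
; BeginPlay caches existing dynamic materials from the hood, bow and arrow; the code that creates them is unconnected.
; PlayVisualEffects fires the particle at the first attacked unit's chest on a successful hit.
; ToggleVisibility flashes emissive, hides bow and arrow, then optionally fades them in via a delay loop as hood glow decays.
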(event Custom|ToggleVisibility
  (params (bShouldAppearance :type Boolean))
  (bind _mi_hood (Variables|Default|GetMI_Hood))
  (for _array_element (Variables|Default|GetMI_Anim)
    (Rendering|Material|SetScalarParameterValue _array_element "EmissiveBoost" 1e+01 :!class /Script/Engine.MaterialInstanceDynamic))
  (Rendering|Material|SetScalarParameterValue (Variables|Default|GetMI_Hood) "EmissiveBoost" 2.5e+02 :!class /Script/Engine.MaterialInstanceDynamic)
  (Utilities|FlowControl|Delay 0.16)
  (for _array_element_2 (Variables|Default|GetMI_Anim)
    (Rendering|Material|SetScalarParameterValue _array_element_2 "OpacityMask" 0.0 :!class /Script/Engine.MaterialInstanceDynamic)
    (Rendering|Material|SetScalarParameterValue _array_element_2 "EmissiveBoost" 1.0 :!class /Script/Engine.MaterialInstanceDynamic))
  (if bShouldAppearance
    (Utilities|FlowControl|Delay 0.2)
    (bind _returnvalue (Rendering|Material|GetScalarParameterValue _mi_hood "EmissiveBoost" :!class /Script/Engine.MaterialInstanceDynamic :!label _label))
    (Rendering|Material|SetScalarParameterValue _mi_hood "EmissiveBoost" (Math|Float|Max(Float) (- _returnvalue 12.5) 1.0) :!class /Script/Engine.MaterialInstanceDynamic)
    (bind _returnvalue_2 (Rendering|Material|GetScalarParameterValue (Utilities|Array|Get(acopy) (Variables|Default|GetMI_Anim)) "OpacityMask" :!class /Script/Engine.MaterialInstanceDynamic))
    (for _array_element_3 (Variables|Default|GetMI_Anim)
      (Rendering|Material|SetScalarParameterValue _array_element_3 "OpacityMask" (+ _returnvalue_2 0.05) :!class /Script/Engine.MaterialInstanceDynamic))
    (if (not (>= (+ _returnvalue_2 0.05) 0.9999))
      (Utilities|FlowControl|Delay 0.05)
      (goto _label))))

(event EventBeginPlay
  (|CallParentFunction)
  (bind _asmaterial_instance_dynamic (Utilities|Casting|CastToMaterialInstanceDynamic (Rendering|Material|GetMaterial (Variables|Default|GetDarkHood) 0)))
  (Variables|Default|SetMI_Hood _asmaterial_instance_dynamic)
  (bind _asmaterial_instance_dynamic_2 (Utilities|Casting|CastToMaterialInstanceDynamic (Rendering|Material|GetMaterial (Variables|Default|GetBow) 0)))
  (Utilities|Array|Add (Variables|Default|GetMI_Anim) _asmaterial_instance_dynamic_2)
  (for _array_element (Rendering|Material|GetMaterials (Variables|Default|GetArrow_0))
    (bind _asmaterial_instance_dynamic_3 (Utilities|Casting|CastToMaterialInstanceDynamic _array_element))
    (Utilities|Array|Add (Variables|Default|GetMI_Anim) _asmaterial_instance_dynamic_3)))

(event EventPlayVisualEffects
  (params (bIsAbilityUsing :type Boolean) (AttackIndex :type Integer))
  (bind _returnvalue (CallFunction|GetAttackResults))
  (if (.bIsSuccessful (Utilities|Struct|BreakS_AttackResult (Utilities|Array|Get(acopy) _returnvalue)))
    (Transformation|SetWorldLocation (Variables|Default|GetP_ImpactEffect) (Default|GetChestSocketLocation (.AttackedUnit (Utilities|Struct|BreakS_AttackResult (Utilities|Array|Get(acopy) _returnvalue)))) false false)
    (Components|Activation|Activate (Variables|Default|GetP_ImpactEffect) true)))

(fn ConstructionScript)