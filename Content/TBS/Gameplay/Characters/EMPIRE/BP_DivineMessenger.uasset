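; Empire Divine Messenger unit for the turn-based battle system, a support character that heals and can resurrect its target as an ability.
; PlayVisualEffects branches on ability use, timing particles with delays and placing them on the first attack result's unit, with the ability path also calling RESURRECTION.
; Trousers and Cape components are briefly nudged during actions, and Trousers on damage.
; Hit calculation always hits without criticals, and damage is the raw Damage stat.
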(event Custom|OnDamageReceived
  (Utilities|FlowControl|Delay 0.35)
  (Transformation|SetRelativeRotation (Variables|Default|GetTrousers) "0, 0,4.000000" false false)
  (Utilities|FlowControl|Delay 1.075)
  (Transformation|SetRelativeRotation (Variables|Default|GetTrousers) "0, 0, 0" false false))

(event EventPlayVisualEffects
  (params (bIsAbilityUsing :type Boolean) (AttackIndex :type Integer))
  (bind _p_resurrection_target (Variables|Default|GetP_Resurrection_Target))
  (if bIsAbilityUsing
    (Components|Activation|Activate (Variables|Default|GetP_AbilityEffect) true)
    (Transformation|SetRelativeLocation (Variables|Default|GetTrousers) "0,2.000000, 0" false false)
    (Transformation|SetRelativeRotation (Variables|Default|GetCape) "0, 0,-0.723845" false false)
    (Utilities|FlowControl|Delay 1.0)
    (bind _returnvalue (CallFunction|GetAttackResults))
    (Transformation|SetWorldLocation _p_resurrection_target (+ (Transformation|GetActorLocation (Utilities|Struct|BreakS_AttackResult (Utilities|Array|Get(acopy) _returnvalue))) "0, 0,100.000000") false false)
    (Default|RESURRECTION (Utilities|Struct|BreakS_AttackResult (Utilities|Array|Get(acopy) _returnvalue)))
    (Components|Activation|Activate _p_resurrection_target true)
    (Utilities|FlowControl|Delay 1.5725)
    (Transformation|SetRelativeLocation (Variables|Default|GetTrousers) "0, 0, 0" false false)
    (Transformation|SetRelativeRotation (Variables|Default|GetCape) "0, 0, 0" false false)
    (else
      (Transformation|SetRelativeLocation (Variables|Default|GetTrousers) "0,10.000000, 0" false false)
      (Transformation|SetRelativeRotation (Variables|Default|GetCape) "0, 0,2.023878" false false)
      (Utilities|FlowControl|Delay 0.75)
      (Components|Activation|Activate (Variables|Default|GetP_HealingEffect_Healer) true)
      (Utilities|FlowControl|Delay 1.25)
      (Transformation|SetRelativeLocation (Variables|Default|GetTrousers) "0, 0, 0" false false)
      (Transformation|SetRelativeRotation (Variables|Default|GetCape) "0, 0, 0" false false)
      (bind _returnvalue_2 (CallFunction|GetAttackResults))
      (Transformation|SetWorldLocation (Variables|Default|GetP_HealingEffect_Target) (- (Transformation|GetActorLocation (Utilities|Struct|BreakS_AttackResult (Utilities|Array|Get(acopy) _returnvalue_2))) "0, 0,95.000000") false false)
      (Transformation|SetWorldScale3D (Variables|Default|GetP_HealingEffect_Target) (select (Default|IsBigUnit (Utilities|Struct|BreakS_AttackResult (Utilities|Array|Get(acopy) _returnvalue_2))) "1.450000,1.450000,1.450000" "1.000000,1.000000,1.000000"))
      (Components|Activation|Activate (Variables|Default|GetP_HealingEffect_Target) true))))

(event EventBeginPlay
  (|CallParentFunction))

(fn ConstructionScript)

(fn CalculateHitorMiss
  (params (AttackedHero :type BP%20Hero%20Base%20Object%20Reference))
  (return true false))

(fn CalculateDamage
  (params (AttackedUnit :type BP%20Hero%20Base%20Object%20Reference) (bIsCritical :type Boolean))
  (return (Utilities|Struct|BreakS_HeroGameplayStats (CallFunction|GetUnitStats))))