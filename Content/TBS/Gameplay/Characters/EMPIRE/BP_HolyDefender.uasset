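; BP_HolyDefender is an Empire character Blueprint in the TBS game, handling the unit's hood material and trail effects.
; On BeginPlay it creates a dynamic material instance for the DarkHood mesh.
; When masked materials are hidden, a delay loop steps EmissiveBoost down to a threshold, then zeroes OpacityMask.
; PlayTrailEffects runs an anim trail between two sockets for under a second.
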(event EventPlayTrailEffects
  (params (AttackType :type Integer))
  (Effects|Particles|Trails|BeginTrails (Variables|Default|GetP_AnimTrailEffect) "S_Trail_01" "S_Trail_02" "ETrailWidthMode_FromCentre" 1.5)
  (Utilities|FlowControl|Delay 0.85)
  (Effects|Particles|Trails|EndTrails (Variables|Default|GetP_AnimTrailEffect)))

(event EventBeginPlay
  (bind _darkhood (Variables|Default|GetDarkHood))
  (|CallParentFunction)
  (bind _returnvalue (Rendering|Material|CreateDynamicMaterialInstance _darkhood 0 (Rendering|Material|GetMaterial _darkhood 0) "None" :!class /Script/Engine.PrimitiveComponent))
  (Variables|Default|SetMI_Hood _returnvalue))

(event EventToggleMaskedMaterials
  (params (bIsVisible :type Boolean))
  (bind _mi_hood (Variables|Default|GetMI_Hood))
  (if (not bIsVisible)
    (bind _returnvalue (Rendering|Material|GetScalarParameterValue _mi_hood "EmissiveBoost" :!class /Script/Engine.MaterialInstanceDynamic :!label _label))
    (Rendering|Material|SetScalarParameterValue _mi_hood "EmissiveBoost" (- _returnvalue 0.075) :!class /Script/Engine.MaterialInstanceDynamic)
    (if (<= (- _returnvalue 0.075) 0.5)
      (Rendering|Material|SetScalarParameterValue (Variables|Default|GetMI_Hood) "OpacityMask" 0.0 :!class /Script/Engine.MaterialInstanceDynamic)
      (else
        (Utilities|FlowControl|Delay 0.075)
        (goto _label)))))

(fn ConstructionScript)