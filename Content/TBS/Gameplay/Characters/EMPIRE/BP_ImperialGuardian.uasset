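; BP_ImperialGuardian is an Empire unit character that adds its own weapon trail and hit-reaction effects on top of its parent Blueprint.
; On BeginPlay it creates dynamic materials for left and right AnimTrail particle components, tinting them gold and storing them in an array.
; PlayTrailEffects runs both socket-based trails for a second.
; PlayVisualEffects plays the first attacked unit's hit animations if that attack succeeded.
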(event EventBeginPlay
  (bind _p_animtraileffect_r (Variables|Default|GetP_AnimTrailEffect_R))
  (bind _p_animtraileffect_l (Variables|Default|GetP_AnimTrailEffect_L))
  (|CallParentFunction)
  (bind _returnvalue (Rendering|Material|CreateDynamicMaterialInstance _p_animtraileffect_l 0 (Rendering|Material|GetMaterial _p_animtraileffect_l 0) "None" :!class /Script/Engine.PrimitiveComponent))
  (Utilities|Array|Add (Variables|Default|GetMI_TrailEffects) _returnvalue)
  (Rendering|Material|SetScalarParameterValue _returnvalue "Opacity" 4.0 :!class /Script/Engine.MaterialInstanceDynamic)
  (Rendering|Material|SetVectorParameterValue _returnvalue "Color" "(R=0.771875,G=0.467735,B=0.044283,A=1.000000)" :!class /Script/Engine.MaterialInstanceDynamic)
  (bind _returnvalue_2 (Rendering|Material|CreateDynamicMaterialInstance _p_animtraileffect_r 0 (Rendering|Material|GetMaterial _p_animtraileffect_r 0) "None" :!class /Script/Engine.PrimitiveComponent))
  (Utilities|Array|Add (Variables|Default|GetMI_TrailEffects) _returnvalue_2)
  (Rendering|Material|SetScalarParameterValue _returnvalue_2 "Opacity" 4.0 :!class /Script/Engine.MaterialInstanceDynamic)
  (Rendering|Material|SetVectorParameterValue _returnvalue_2 "Color" "(R=1.000000,G=0.605973,B=0.057371,A=1.000000)" :!class /Script/Engine.MaterialInstanceDynamic))

(event EventPlayTrailEffects
  (params (AttackType :type Integer))
  (Effects|Particles|Trails|BeginTrails (Variables|Default|GetP_AnimTrailEffect_L) "S_Trail_01_L" "S_Trail_02_L" "ETrailWidthMode_FromCentre" 3.0)
  (Effects|Particles|Trails|BeginTrails (Variables|Default|GetP_AnimTrailEffect_R) "S_Trail_01_R" "S_Trail_02_R" "ETrailWidthMode_FromCentre" 3.0)
  (Utilities|FlowControl|Delay 1.0)
  (Effects|Particles|Trails|EndTrails (Variables|Default|GetP_AnimTrailEffect_L)))

(event EventPlayVisualEffects
  (params (bIsAbilityUsing :type Boolean) (AttackIndex :type Integer))
  (bind _returnvalue (CallFunction|GetAttackResults))
  (if (.bIsSuccessful (Utilities|Struct|BreakS_AttackResult (Utilities|Array|Get(acopy) _returnvalue)))
    (Default|PlayHitAnimations (.AttackedUnit (Utilities|Struct|BreakS_AttackResult (Utilities|Array|Get(acopy) _returnvalue))))))

(fn ConstructionScript)