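; BP_Ranger is the Empire archer unit in the TBS game, adding bow attack visuals and a critical-hit rule to its parent character.
; PlayVisualEffects times the arrow's visibility and swaps three bowstring meshes through delays to fake the draw and release.
; If the first attack result succeeds, it moves the arrow effect to the target's chest socket and activates it.
; CalculateIsCriticalAttack rolls randomly against a hit-value-based chance with a minimum floor.
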(event Custom|ToggleBowstring
  (params (Index :type Integer))
  (switch int Index
    (:0
      (Development|SetHiddeninGame (Variables|Default|GetBowstring_Attack_1) true false)
      (Development|SetHiddeninGame (Variables|Default|GetBowstring) false false))
    (:1
      (Development|SetHiddeninGame (Variables|Default|GetBowstring_Attack_2) true false)
      (Development|SetHiddeninGame (Variables|Default|GetBowstring_Attack_1) false false))
    (:2
      (Development|SetHiddeninGame (Variables|Default|GetBowstring_Attack_1) true false)
      (Development|SetHiddeninGame (Variables|Default|GetBowstring_Attack_2) false false))))

(event EventBeginPlay
  (|CallParentFunction))

(event EventPlayVisualEffects
  (params (bIsAbilityUsing :type Boolean) (AttackIndex :type Integer))
  (Development|SetHiddeninGame (Variables|Default|GetArrow_0) false false)
  (Utilities|FlowControl|Delay 0.32)
  (CallFunction|ToggleBowstring 1)
  (Utilities|FlowControl|Delay 0.195)
  (CallFunction|ToggleBowstring 2)
  (Utilities|FlowControl|Delay 0.3865)
  (Development|SetHiddeninGame (Variables|Default|GetArrow_0) true false)
  (CallFunction|ToggleBowstring)
  (bind _returnvalue (CallFunction|GetAttackResults))
  (if (.bIsSuccessful (Utilities|Struct|BreakS_AttackResult (Utilities|Array|Get(acopy) _returnvalue)))
    (Utilities|FlowControl|Delay 0.15)
    (Transformation|SetWorldLocation (Variables|Default|GetP_Archer_Arrow) (Default|GetChestSocketLocation (.AttackedUnit (Utilities|Struct|BreakS_AttackResult (Utilities|Array|Get(acopy) _returnvalue)))) false false)
    (Components|Activation|Activate (Variables|Default|GetP_Archer_Arrow) true)))

(fn ConstructionScript)

(fn CalculateIsCriticalAttack
  (params (AttackedHero :type BP%20Hero%20Base%20Object%20Reference) (HitValue :type Float%20%28single-precision%29))
  (return (> (Math|Float|Max(Float) (- HitValue 0.595) 0.05) (- (Math|Random|RandomFloat) 0.0675))))