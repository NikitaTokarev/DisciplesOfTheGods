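; BP_Misrail is an Empire character Blueprint in the turn-based strategy game, with a lightning effect for its attack visuals.
; PlayVisualEffects reads the attack results, teleport-free moves PLightningEffect to 90 units below the first attacked unit's location, and activates it with a reset.
; Only the first target receives the effect; BeginPlay just calls the parent, and the construction script is empty.
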(event EventBeginPlay
  (|CallParentFunction))

(event EventPlayVisualEffects
  (params (bIsAbilityUsing :type Boolean) (AttackIndex :type Integer))
  (bind _returnvalue (CallFunction|GetAttackResults))
  (Transformation|SetWorldLocation (Variables|Default|GetP_LightningEffect) (- (Transformation|GetActorLocation (Utilities|Struct|BreakS_AttackResult (Utilities|Array|Get(acopy) _returnvalue))) "0, 0,90.000000") false false)
  (Components|Activation|Activate (Variables|Default|GetP_LightningEffect) true))

(fn ConstructionScript)