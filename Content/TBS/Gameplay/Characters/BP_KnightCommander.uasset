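; BP_KnightCommander is the Knight Commander character Blueprint for the TBS game, adding weapon trail and ability visual effects to its parent class.
; BeginPlay creates a dynamic material instance on the AnimTrail particle component so trail opacity can vary by attack type.
; PlayTrailEffects sets that opacity, runs the trail between two sockets and ends it after a fixed delay.
; PlayVisualEffects activates the ability particle effect.
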(event EventPlayTrailEffects
  (params (AttackType :type Integer))
  (Rendering|Material|SetScalarParameterValue (Variables|Default|GetMI_TrailEffect) "Opacity" (Utilities|Select :Index AttackType :Option%200 1.0 :Option%201 3.0) :!class /Script/Engine.MaterialInstanceDynamic)
  (Effects|Particles|Trails|BeginTrails (Variables|Default|GetP_AnimTrailEffect) "S_Trail_01" "S_Trail_02" "ETrailWidthMode_FromCentre" 1.5)
  (Utilities|FlowControl|Delay 0.85)
  (Effects|Particles|Trails|EndTrails (Variables|Default|GetP_AnimTrailEffect)))

(event EventBeginPlay
  (bind _p_animtraileffect (Variables|Default|GetP_AnimTrailEffect))
  (|CallParentFunction)
  (bind _returnvalue (Rendering|Material|CreateDynamicMaterialInstance _p_animtraileffect 0 (Rendering|Material|GetMaterial _p_animtraileffect 0) "None" :!class /Script/Engine.PrimitiveComponent))
  (Variables|Default|SetMI_TrailEffect _returnvalue))

(event EventPlayVisualEffects
  (params (bIsAbilityUsing :type Boolean) (AttackIndex :type Integer))
  (Components|Activation|Activate (Variables|Default|GetP_AbilityEffect) true))

(fn ConstructionScript)