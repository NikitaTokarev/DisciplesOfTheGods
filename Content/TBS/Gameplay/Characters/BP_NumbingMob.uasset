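; BP_NumbingMob is a turn-based strategy mob character whose attack does no damage calculation.
; ShouldCalculateDamage always returns false.
; PlayVisualEffects moves the attack particle to just below the first attacked unit's location from the attack results, then activates it.
; The numbing effect implied by the name is not implemented in this graph.
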(event EventBeginPlay
  (|CallParentFunction) ; This node is disabled and will not be called.\nDrag off pins to build functionality.
)

(event EventPlayVisualEffects
  (params (bIsAbilityUsing :type Boolean))
  (bind _returnvalue (CallFunction|GetAttackResults))
  (Transformation|SetWorldLocation (Variables|Default|GetP_AttackParticle) (- (Transformation|GetActorLocation (.AttackedUnit (Utilities|Struct|BreakS_AttackResult (Utilities|Array|Get(acopy) _returnvalue)))) "0, 0,110.000000") false false)
  (Components|Activation|Activate (Variables|Default|GetP_AttackParticle) true))

(fn ConstructionScript
  (|CallParentFunction))

(fn ShouldCalculateDamage
  (return false))