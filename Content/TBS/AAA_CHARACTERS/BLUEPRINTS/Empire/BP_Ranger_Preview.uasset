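; Preview actor for the Empire Ranger that endlessly replays the bow attack montage.
; BeginPlay starts the loop after a short delay, waiting out each montage's length plus a pause before repeating.
; A separate Attack event, with no caller in these graphs, shows the arrow and uses timed delays to fake the draw.
; ToggleBowstring swaps visibility between resting and two attack bowstring components, then Attack restores rest and hides the arrow.
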(event Custom|Attack
  (Development|SetHiddeninGame (Variables|Default|GetArrow) false false)
  (Utilities|FlowControl|Delay 0.32)
  (CallFunction|ToggleBowstring 1)
  (Utilities|FlowControl|Delay 0.195)
  (CallFunction|ToggleBowstring 2)
  (Utilities|FlowControl|Delay 0.3865)
  (Development|SetHiddeninGame (Variables|Default|GetArrow) true false)
  (CallFunction|ToggleBowstring))

(event Custom|ToggleBowstring
  (params (Index :type Integer))
  (switch int Index
    (:0
      (Development|SetHiddeninGame (Variables|Default|GetBowstring_Attack_1) true false)
      (Development|SetHiddeninGame (Variables|Default|GetBowstring) false false))
    (:1
      (Development|SetHiddeninGame (Variables|Default|GetBowstring_Attack_2) true false)
      (Development|SetHiddeninGame (Variables|Default|GetBowstring_Attack_1) false false))
    (:2
      (Development|SetHiddeninGame (Variables|Default|GetBowstring_Attack_1) true false)
      (Development|SetHiddeninGame (Variables|Default|GetBowstring_Attack_2) false false))))

(event EventBeginPlay
  (Utilities|FlowControl|Delay 1.0 :!label _label)
  (bind _returnvalue (Animation|Montage|MontagePlay (Components|SkeletalMesh|GetAnimInstance (Variables|Default|GetSkeletalMesh)) "/Game/TBS/AAA_CHARACTERS/CHARACTERS/Empire/Ranger/Animations/Montages/AM_Ranger_Attack.AM_Ranger_Attack" 1.0 "MontageLength" 0.0 true))
  (Utilities|FlowControl|Delay (+ _returnvalue 1.75))
  (goto _label))

(fn ConstructionScript)