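; BP_DivineMessenger is the Empire Divine Messenger healer character, handling its animation playback and timed visual effects.
; BeginPlay endlessly plays a random Ability or Healing montage, waiting the montage length plus a pause between plays.
; Attack fires healer then target healing effects, while Ability fires its own effect.
; Attack, Ability and OnHit temporarily offset or rotate the trousers or cape meshes, using hard-coded delays before resetting them.
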(event Custom|Attack
  (Transformation|SetRelativeLocation (Variables|Default|GetTrousers) "0,10.000000, 0" false false)
  (Transformation|SetRelativeRotation (Variables|Default|GetCape) "0, 0,2.023878" false false)
  (Utilities|FlowControl|Delay 0.75)
  (Components|Activation|Activate (Variables|Default|GetP_HealingEffect_Healer) true)
  (Utilities|FlowControl|Delay 1.25)
  (Transformation|SetRelativeLocation (Variables|Default|GetTrousers) "0, 0, 0" false false)
  (Transformation|SetRelativeRotation (Variables|Default|GetCape) "0, 0, 0" false false)
  (Components|Activation|Activate (Variables|Default|GetP_HealingEffect_Target) true))

(event Custom|Ability
  (Components|Activation|Activate (Variables|Default|GetP_AbilityEffect) true)
  (Transformation|SetRelativeLocation (Variables|Default|GetTrousers) "0,2.000000, 0" false false)
  (Transformation|SetRelativeRotation (Variables|Default|GetCape) "0, 0,-0.723845" false false)
  (Utilities|FlowControl|Delay 2.5725)
  (Transformation|SetRelativeLocation (Variables|Default|GetTrousers) "0, 0, 0" false false)
  (Transformation|SetRelativeRotation (Variables|Default|GetCape) "0, 0, 0" false false))

(event Custom|OnHit
  (Utilities|FlowControl|Delay 0.35)
  (Transformation|SetRelativeRotation (Variables|Default|GetTrousers) "0, 0,4.000000" false false)
  (Utilities|FlowControl|Delay 1.075)
  (Transformation|SetRelativeRotation (Variables|Default|GetTrousers) "0, 0, 0" false false))

(event EventBeginPlay
  (Utilities|FlowControl|Delay 1.0)
  (bind _returnvalue (Animation|Montage|MontagePlay (Components|SkeletalMesh|GetAnimInstance (Variables|Default|GetSkeletalMesh)) (select (Math|Random|RandomBool) "/Game/TBS/AAA_CHARACTERS/CHARACTERS/Empire/DivineMessenger/Animations/Montages/AM_DivineMessenger_Ability.AM_DivineMessenger_Ability" "/Game/TBS/AAA_CHARACTERS/CHARACTERS/Empire/DivineMessenger/Animations/Montages/AM_DivineMessenger_Healing.AM_DivineMessenger_Healing") 1.0 "MontageLength" 0.0 true :!label _label))
  (Utilities|FlowControl|Delay (+ _returnvalue 3.0))
  (goto _label))

(fn ConstructionScript)