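; Preview actor for the Empire Assassin that replays its attack montage in an endless loop to show off the teleport strike.
; BeginPlay stores the original transform, tints the trail's dynamic material and starts the montage loop.
; PlayAttackEffect uses delays to sequence smoke and beam particles, visibility toggles, and a jump to an offset, turned-around position and back.
; TrailEffect briefly runs an anim trail between two sockets; neither event is called within this graph.
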(event Custom|TrailEffect
  (Effects|Particles|Trails|BeginTrails (Variables|Default|GetP_AnimTrailEffect) "S_Trail_01" "S_Trail_02" "ETrailWidthMode_FromCentre" 1.5)
  (Utilities|FlowControl|Delay 0.4)
  (Effects|Particles|Trails|EndTrails (Variables|Default|GetP_AnimTrailEffect)))

(event Custom|PlayAttackEffect
  (bind _originaltransform (Variables|Default|GetOriginalTransform))
  (bind _originaltransform_2 (Variables|Default|GetOriginalTransform))
  (bind (_location _rotation) (Math|Transform|BreakTransform _originaltransform))
  (Components|Activation|Activate (Variables|Default|GetP_TeleportEffect_Smoke) true)
  (Utilities|FlowControl|Delay 0.075)
  (Transformation|SetActorLocationAndRotation (+ "0,-400.000000, 0" _location) (Math|Rotator|MakeRotator (.roll _rotation) (.pitch _rotation) (+ (.yaw _rotation) 1.8e+02)))
  (Components|Activation|Activate (Variables|Default|GetP_TeleportEffect_Beam) true)
  (Utilities|FlowControl|Delay 0.15)
  (Development|SetHiddeninGame (Variables|Default|GetSkeletalMesh) false true)
  (Utilities|FlowControl|Delay 1.6)
  (Components|Activation|Activate (Variables|Default|GetP_TeleportEffect_Smoke) true)
  (Development|SetHiddeninGame (Variables|Default|GetSkeletalMesh) true true)
  (Utilities|FlowControl|Delay 0.875)
  (Transformation|SetActorLocationAndRotation (.location _originaltransform_2) (.rotation _originaltransform_2))
  (Components|Activation|Activate (Variables|Default|GetP_TeleportEffect_Smoke) true)
  (Development|SetHiddeninGame (Variables|Default|GetSkeletalMesh) false true))

(event EventBeginPlay
  (bind _p_animtraileffect (Variables|Default|GetP_AnimTrailEffect))
  (Variables|Default|SetOriginalTransform (Transformation|GetActorTransform))
  (bind _returnvalue (Rendering|Material|CreateDynamicMaterialInstance _p_animtraileffect 0 (Rendering|Material|GetMaterial _p_animtraileffect 0) "None" :!class /Script/Engine.PrimitiveComponent))
  (bind _output_get (Variables|Default|SetMI_TrailEffect _returnvalue))
  (Rendering|Material|SetScalarParameterValue _output_get "Opacity" 4.0 :!class /Script/Engine.MaterialInstanceDynamic)
  (Rendering|Material|SetVectorParameterValue _output_get "Color" "(R=0.116580,G=0.004881,B=0.575000,A=1.000000)" :!class /Script/Engine.MaterialInstanceDynamic)
  (Utilities|FlowControl|Delay 1.0)
  (bind _returnvalue_2 (Animation|Montage|MontagePlay (Components|SkeletalMesh|GetAnimInstance (Variables|Default|GetSkeletalMesh)) "/Game/TBS/AAA_CHARACTERS/CHARACTERS/Empire/Assassin/Animations/Montages/AM_Assassin_Attack_01.AM_Assassin_Attack_01" 1.0 "MontageLength" 0.0 true :!label _label))
  (Utilities|FlowControl|Delay (+ _returnvalue_2 1.5))
  (goto _label))

(fn ConstructionScript)