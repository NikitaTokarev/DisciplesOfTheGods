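; Preview actor for the Empire Imperial Knight that plays its attack animation on a repeating loop.
; After a one-second delay on BeginPlay it plays the attack montage, waits for its length plus a pause, then repeats.
; A TrailEffect event runs an anim trail between two sockets for one second.
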(event Custom|TrailEffect
  (Effects|Particles|Trails|BeginTrails (Variables|Default|GetP_AnimTrail_Effect) "S_Trail_01" "S_Trail_02" "ETrailWidthMode_FromCentre" 1.5)
  (Utilities|FlowControl|Delay 1.0)
  (Effects|Particles|Trails|EndTrails (Variables|Default|GetP_AnimTrail_Effect)))

(event EventBeginPlay
  (Utilities|FlowControl|Delay 1.0)
  (bind _returnvalue (Animation|Montage|MontagePlay (Components|SkeletalMesh|GetAnimInstance (Variables|Default|GetSkeletalMesh)) "/Game/TBS/AAA_CHARACTERS/CHARACTERS/Empire/ImperialKnight/Animations/Montages/AM_ImperialKnight_Attack.AM_ImperialKnight_Attack" 1.0 "MontageLength" 0.0 true :!label _label))
  (Utilities|FlowControl|Delay (+ _returnvalue 1.75))
  (goto _label))

(fn ConstructionScript)