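; Knight Commander character Blueprint for the Empire set, which loops randomly chosen attack and ability montages as an automatic animation showcase.
; BeginPlay creates a dynamic trail material, then repeatedly plays a montage, waiting out its length plus a pause.
; TrailEffect sets trail opacity by attack type and runs an anim trail between two sockets for a fixed window.
; AbilityEffect activates the ability particle effect.
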(event Custom|TrailEffect
  (params (AttackType :type Integer))
  (Rendering|Material|SetScalarParameterValue (Variables|Default|GetMI_TrailEffect) "Opacity" (Utilities|Select :Index AttackType :Option%200 1.0 :Option%201 3.0) :!class /Script/Engine.MaterialInstanceDynamic)
  (Effects|Particles|Trails|BeginTrails (Variables|Default|GetP_AnimTrailEffect) "S_Trail_01" "S_Trail_02" "ETrailWidthMode_FromCentre" 1.5)
  (Utilities|FlowControl|Delay 0.85)
  (Effects|Particles|Trails|EndTrails (Variables|Default|GetP_AnimTrailEffect)))

(event Custom|AbilityEffect
  (Components|Activation|Activate (Variables|Default|GetP_AbilityEffect) true))

(event EventBeginPlay
  (bind _p_animtraileffect (Variables|Default|GetP_AnimTrailEffect))
  (bind _returnvalue (Rendering|Material|CreateDynamicMaterialInstance _p_animtraileffect 0 (Rendering|Material|GetMaterial _p_animtraileffect 0) "None" :!class /Script/Engine.PrimitiveComponent))
  (Variables|Default|SetMI_TrailEffect _returnvalue)
  (Utilities|FlowControl|Delay 1.0)
  (bind _returnvalue_2 (Animation|Montage|MontagePlay (Components|SkeletalMesh|GetAnimInstance (Variables|Default|GetSkeletalMesh)) (Utilities|Select :Index (Math|Random|RandomIntegerinRange 0 3) :Option%200 "/Game/TBS/AAA_CHARACTERS/CHARACTERS/Empire/KnightCommander/Animations/Montages/AM_KnightCommander_Attack_01.AM_KnightCommander_Attack_01" :Option%201 "/Game/TBS/AAA_CHARACTERS/CHARACTERS/Empire/KnightCommander/Animations/Montages/AM_KnightCommander_Attack_02.AM_KnightCommander_Attack_02" :Option%202 "/Game/TBS/AAA_CHARACTERS/CHARACTERS/Empire/KnightCommander/Animations/Montages/AM_KnightCommander_Attack_03.AM_KnightCommander_Attack_03" :Option%203 "/Game/TBS/AAA_CHARACTERS/CHARACTERS/Empire/KnightCommander/Animations/Montages/AM_KnightCommander_Ability.AM_KnightCommander_Ability") 1.0 "MontageLength" 0.0 true :!label _label))
  (Utilities|FlowControl|Delay (+ _returnvalue_2 1.75))
  (goto _label))

(fn ConstructionScript)