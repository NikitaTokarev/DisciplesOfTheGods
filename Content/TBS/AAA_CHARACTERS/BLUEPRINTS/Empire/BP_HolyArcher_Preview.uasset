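; BP_HolyArcher_Preview is a preview actor for the Empire Holy Archer that endlessly replays its attack montage with a pause between plays.
; BeginPlay creates dynamic material instances for the hood, bow and arrow.
; ToggleVisibility flashes their emissive boost, then hides bow and arrow through an opacity mask parameter.
; When appearance is requested, a Delay-driven loop fades bow and arrow back in while stepping down the hood's glow.
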(event Custom|ToggleVisibility
  (params (bShouldAppearance :type Boolean))
  (bind _mi_hood (Variables|Default|GetMI_Hood))
  (for _array_element (Variables|Default|GetMI_Anim)
    (Rendering|Material|SetScalarParameterValue _array_element "EmissiveBoost" 2.5e+02 :!class /Script/Engine.MaterialInstanceDynamic))
  (Rendering|Material|SetScalarParameterValue (Variables|Default|GetMI_Hood) "EmissiveBoost" 2.5e+02 :!class /Script/Engine.MaterialInstanceDynamic)
  (Utilities|FlowControl|Delay 0.16)
  (for _array_element_2 (Variables|Default|GetMI_Anim)
    (Rendering|Material|SetScalarParameterValue _array_element_2 "OpacityMask" 0.0 :!class /Script/Engine.MaterialInstanceDynamic)
    (Rendering|Material|SetScalarParameterValue _array_element_2 "EmissiveBoost" 1.0 :!class /Script/Engine.MaterialInstanceDynamic))
  (if bShouldAppearance
    (Utilities|FlowControl|Delay 0.2)
    (bind _returnvalue (Rendering|Material|GetScalarParameterValue _mi_hood "EmissiveBoost" :!class /Script/Engine.MaterialInstanceDynamic :!label _label))
    (Rendering|Material|SetScalarParameterValue _mi_hood "EmissiveBoost" (Math|Float|Max(Float) (- _returnvalue 12.5) 1.0) :!class /Script/Engine.MaterialInstanceDynamic)
    (bind _returnvalue_2 (Rendering|Material|GetScalarParameterValue (Utilities|Array|Get(acopy) (Variables|Default|GetMI_Anim)) "OpacityMask" :!class /Script/Engine.MaterialInstanceDynamic))
    (for _array_element_3 (Variables|Default|GetMI_Anim)
      (Rendering|Material|SetScalarParameterValue _array_element_3 "OpacityMask" (+ _returnvalue_2 0.05) :!class /Script/Engine.MaterialInstanceDynamic))
    (if (not (>= (+ _returnvalue_2 0.05) 0.9999))
      (Utilities|FlowControl|Delay 0.05)
      (goto _label))))

(event EventBeginPlay
  (bind _darkhood (Variables|Default|GetDarkHood))
  (bind _bow (Variables|Default|GetBow))
  (bind _returnvalue (Rendering|Material|CreateDynamicMaterialInstance _darkhood 0 (Rendering|Material|GetMaterial _darkhood 0) "None" :!class /Script/Engine.PrimitiveComponent))
  (Variables|Default|SetMI_Hood _returnvalue)
  (bind _returnvalue_2 (Rendering|Material|CreateDynamicMaterialInstance _bow 0 (Rendering|Material|GetMaterial _bow 0) "None" :!class /Script/Engine.PrimitiveComponent))
  (Utilities|Array|Add (Variables|Default|GetMI_Anim) _returnvalue_2)
  (for (_array_element _array_index) (Rendering|Material|GetMaterials (Variables|Default|GetArrow))
    (bind _returnvalue_3 (Rendering|Material|CreateDynamicMaterialInstance (Variables|Default|GetArrow) _array_index _array_element "None" :!class /Script/Engine.PrimitiveComponent))
    (Utilities|Array|Add (Variables|Default|GetMI_Anim) _returnvalue_3))
  (Utilities|FlowControl|Delay 1.0)
  (bind _returnvalue_4 (Animation|Montage|MontagePlay (Components|SkeletalMesh|GetAnimInstance (Variables|Default|GetSkeletalMesh)) "/Game/TBS/AAA_CHARACTERS/CHARACTERS/Empire/HolyArcher/Animations/Montages/AM_HolyArcher_Attack.AM_HolyArcher_Attack" 1.0 "MontageLength" 0.0 true :!label _label))
  (Utilities|FlowControl|Delay (+ _returnvalue_4 1.0))
  (goto _label))

(fn ConstructionScript)