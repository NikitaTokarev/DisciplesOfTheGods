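; Preview Blueprint for the Empire Master of the Blade character that replays its attack montage in an endless loop.
; BeginPlay creates a tinted dynamic material for the anim-trail particle component, then repeats the montage with a pause after each play.
; A separate TrailEffect event, with no caller in this graph, briefly runs a weapon trail between two sockets using Begin/EndTrails.
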(event Custom|TrailEffect
  (Effects|Particles|Trails|BeginTrails (Variables|Default|GetP_AnimTrailEffect) "S_Trail_01" "S_Trail_02" "ETrailWidthMode_FromCentre" 1.5)
  (Utilities|FlowControl|Delay 0.4)
  (Effects|Particles|Trails|EndTrails (Variables|Default|GetP_AnimTrailEffect)))

(event EventBeginPlay
  (bind _p_animtraileffect (Variables|Default|GetP_AnimTrailEffect))
  (bind _returnvalue (Rendering|Material|CreateDynamicMaterialInstance _p_animtraileffect 0 (Rendering|Material|GetMaterial _p_animtraileffect 0) "None" :!class /Script/Engine.PrimitiveComponent))
  (bind _output_get (Variables|Default|SetMI_TrailEffect _returnvalue))
  (Rendering|Material|SetScalarParameterValue _output_get "Opacity" 4.0 :!class /Script/Engine.MaterialInstanceDynamic)
  (Rendering|Material|SetVectorParameterValue _output_get "Color" "(R=0.468753,G=0.510729,B=0.771875,A=1.000000)" :!class /Script/Engine.MaterialInstanceDynamic)
  (Utilities|FlowControl|Delay 1.0)
  (bind _returnvalue_2 (Animation|Montage|MontagePlay (Components|SkeletalMesh|GetAnimInstance (Variables|Default|GetSkeletalMesh)) "/Game/TBS/AAA_CHARACTERS/CHARACTERS/Empire/MasterOfTheBlade/Animations/Montages/AM_MasterOfTheBlade_Attack.AM_MasterOfTheBlade_Attack" 1.0 "MontageLength" 0.0 true :!label _label))
  (Utilities|FlowControl|Delay (+ _returnvalue_2 1.5))
  (goto _label))

(fn ConstructionScript)