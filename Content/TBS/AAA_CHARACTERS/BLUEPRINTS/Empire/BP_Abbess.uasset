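; BP_Abbess is an Empire character Blueprint for the Abbess that cycles through her ability and healing animations.
; After a one-second delay from BeginPlay, it endlessly plays a randomly chosen montage, waiting for the montage length plus one second between plays.
; Two separate events activate the heal and ability particle effects; the loop itself does not call them.
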(event Custom|PlayEffects_Heal
  (Components|Activation|Activate (Variables|Default|GetP_HealingEffect) true))

(event Custom|PlayEffects_Ability
  (Components|Activation|Activate (Variables|Default|GetP_AbilityEffect) true))

(event EventBeginPlay
  (Utilities|FlowControl|Delay 1.0)
  (bind _returnvalue (Animation|Montage|MontagePlay (Components|SkeletalMesh|GetAnimInstance (Variables|Default|GetSkeletalMesh)) (select (Math|Random|RandomBool) "/Game/TBS/AAA_CHARACTERS/CHARACTERS/Empire/Abbess/Animations/Montages/AM_Abbess_Ability.AM_Abbess_Ability" "/Game/TBS/AAA_CHARACTERS/CHARACTERS/Empire/Abbess/Animations/Montages/AM_Abbess_Healing.AM_Abbess_Healing") 1.0 "MontageLength" 0.0 true :!label _label))
  (Utilities|FlowControl|Delay (+ _returnvalue 1.0))
  (goto _label))

(fn ConstructionScript)