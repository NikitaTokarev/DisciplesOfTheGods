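; BP_AIController_Group is a group-level AI controller that coordinates a set of units in the turn-based strategy game.
; It registers each added unit and initializes that unit's own controller with references to the group and unit.
; Turn starts are forwarded to unit controllers through message calls, while turn switches call CycleTurns on the cached TBSGameMode.
; EndTurn is an empty stub.
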(event EventBeginPlay
  (bind _astbsgame_mode (Utilities|Casting|CastToTBSGameMode (Game|GetGameMode)))
  (Variables|Default|SetGameMode _astbsgame_mode))

(event EventEndTurn)

(event EventStartTurn
  (params (Unit :type BP%20Hero%20Base%20Object%20Reference) (Group0 :type Array%20of%20BP%20Hero%20Base%20Object%20References) (Group1 :type Array%20of%20BP%20Hero%20Base%20Object%20References))
  (Class|BPIUnitController|StartUnitTurn(Message) (Pawn|GetController Unit)))

(event EventAddUnitinGroup
  (params (Unit :type BP%20Hero%20Base%20Object%20Reference))
  (Utilities|Array|Add (Variables|Default|GetGroup) Unit)
  (Class|BPIUnitController|InitializeUnitController(Message) (Pawn|GetController Unit) self Unit))

(event EventSwitchTurn
  (Default|CycleTurns (Variables|Default|GetGameMode)))

(fn ConstructionScript)