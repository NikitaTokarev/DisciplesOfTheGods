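; BP_AIController_UnitBase is the base AI controller for a single unit in the turn-based tactics game, linked to a group controller.
; On its turn it asks the controlled unit for available targets from two groups and makes it attack the first one via a server call, without an ability.
; With no targets, it prints a debug message, waits briefly and tells the group controller to switch turns.
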(event Custom|SelectBestAction
  (params (AvailableTargets :type Array%20of%20BP%20Hero%20Base%20Object%20References))
  ;[1 0.1445 0.09873 1 72] MAIN
  (Default|AttackTargetSERVER (Variables|Default|GetControlledUnit) (Utilities|Array|Get(acopy) AvailableTargets) false))

(event EventStartUnitTurn
  (params (Group0 :type Array%20of%20BP%20Hero%20Base%20Object%20References) (Group1 :type Array%20of%20BP%20Hero%20Base%20Object%20References))
  ;[1 0.1445 0.09873 1 72] MAIN
  (bind _availabletargets (Default|GetAvailableTargets (Variables|Default|GetControlledUnit) Group0 Group1))
  (if (!= (Utilities|Array|Length _availabletargets) 0)
    (CallFunction|SelectBestAction _availabletargets)
    (else
      (Development|PrintString "AI Controller Turn" true true "(R=0.000000,G=1.000000,B=0.289482,A=1.000000)" 4.0)
      (Utilities|FlowControl|Delay 1.0)
      (Class|BPIGroupController|SwitchTurn(Message) (Variables|Default|GetGroupController)))))

(event EventInitializeUnitController
  (params (GroupController :type Controller%20Object%20Reference) (ControlledUnit :type BP%20Hero%20Base%20Object%20Reference))
  ;[1 0.5434 0.8081 1 32] Initializing
  (Variables|Default|SetGroupController GroupController)
  (Variables|Default|SetControlledUnit ControlledUnit))

(fn ConstructionScript)