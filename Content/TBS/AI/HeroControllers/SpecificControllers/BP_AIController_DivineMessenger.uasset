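; AI controller for the Divine Messenger hero in the turn-based game, adding resurrection to the parent's action selection.
; When the ability is available, it casts it on a dead unit from its player's original group, otherwise deferring to parent logic.
; The search skips Holy Archer, Holy Defender and Living Armor.
; It compares base priority against a never-updated maximum, so the last unit above that threshold wins, not necessarily the highest.
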(event EventBeginPlay
  (|CallParentFunction) ; This node is disabled and will not be called.\nDrag off pins to build functionality.
)

(event EventSelectBestAction
  (if (Default|GetCanUseAbility (Variables|Default|GetControlledUnit))
    (bind _returnvalue (CallFunction|HasTargettoResurrect))
    (Utilities|IsValid _returnvalue
      (:Is%20Valid
        (Default|AttackTargetSERVER (Variables|Default|GetControlledUnit) _returnvalue true))
      (:Is%20Not%20Valid
        (|CallParentFunction)))
    (else
      (|CallParentFunction))))

(fn ConstructionScript
  (|CallParentFunction))

(fn HasTargettoResurrect
  (bind (_group0 _group1) (Class|BPIGameState|GetOriginalGroups(Message) (Game|GetGameState)))
  (for _array_element (Utilities|Select :Index (Default|GetPlayerIndex (Variables|Default|GetControlledUnit)) :Option%200 _group0 :Option%201 _group1)
    (if (and (Default|GetIsDead _array_element) (Math|Boolean|ANDBoolean (!= (Utilities|GetClass _array_element) "/Game/TBS/Gameplay/Characters/EMPIRE/BP_HolyArcher.BP_HolyArcher_C") (!= (Utilities|GetClass _array_element) "/Game/TBS/Gameplay/Characters/EMPIRE/BP_HolyDefender.BP_HolyDefender_C") (!= (Utilities|GetClass _array_element) "/Game/TBS/Gameplay/Characters/EMPIRE/BP_LivingArmor.BP_LivingArmor_C")))
      (if (> (Default|GetUnitBasePriority _array_element) (LocalVariables|GetL_MaxPriority))
        (LocalVariables|SetL_Unit _array_element))))
  (return (LocalVariables|GetL_Unit)))