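; Base AI controller for a unit in the turn-based battle, initialized with its group controller and controlled unit.
; On turn start it gathers attack and ability targets from the unit, defends if both are empty, otherwise calls SelectBestAction.
; The default action normally attacks the first available target, ignoring ability targets.
; Helpers for highest-priority target and a constant efficiency factor exist but are unused here.
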(event Custom|SelectBestAction
  ;[1 0.1445 0.09873 1 72] MAIN
  (Default|AttackTargetSERVER (Variables|Default|GetControlledUnit) (Utilities|Array|Get(acopy) (Variables|Default|GetAvailableTargets)) false))

(event EventStartUnitTurn
  (params (Group0 :type Array%20of%20BP%20Hero%20Base%20Object%20References) (Group1 :type Array%20of%20BP%20Hero%20Base%20Object%20References))
  ;[1 0.1445 0.09873 1 72] MAIN
  (bind (_availabletargets _targetsforability) (Default|GetAvailableTargets (Variables|Default|GetControlledUnit) Group0 Group1))
  (bind _output_get (Variables|Default|SetAvailableTargets _availabletargets))
  (bind _output_get_2 (Variables|Default|SetTargetsForAbility _targetsforability))
  (if (or (!= (Utilities|Array|Length _output_get_2) 0) (!= (Utilities|Array|Length _output_get) 0))
    (CallFunction|SelectBestAction)
    (else
      (Default|DefendSERVER (Variables|Default|GetControlledUnit)))))

(event EventInitializeUnitController
  (params (GroupController :type Controller%20Object%20Reference) (ControlledUnit :type BP%20Hero%20Base%20Object%20Reference))
  ;[1 0.5434 0.8081 1 32] Initializing
  (Variables|Default|SetGroupController GroupController)
  (Variables|Default|SetControlledUnit ControlledUnit))

(fn ConstructionScript)

(fn GetTargetwithMaxPriority
  (params (Targets :type Array%20of%20BP%20Hero%20Base%20Object%20References))
  (for _array_element Targets
    (if (> (Default|GetUnitPriority _array_element) (LocalVariables|GetL_MaxPriority))
      (LocalVariables|SetL_MaxPriority (Default|GetUnitPriority _array_element))
      (LocalVariables|SetL_Unit _array_element)))
  (return (LocalVariables|GetL_Unit)))

(fn GetEfficiencyFactor
  (params (TargetUnit :type BP%20Hero%20Base%20Object%20Reference))
  (return 1.0))