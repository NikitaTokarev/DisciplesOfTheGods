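; AI controller for ranged heroes in a turn-based strategy game that picks and attacks the most valuable target.
; SelectBestAction checks whether to use the ability, then chooses from either the ability targets or the available targets.
; GetTargetWithMaxPriority scores each candidate with CalculateEffectivnessOfAttack and returns the highest.
; The controlled unit then attacks that target through AttackTargetSERVER, with or without the ability.
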(event EventBeginPlay)

(event EventSelectBestAction
  (bind _returnvalue (CallFunction|ShouldUseAbility))
  (if _returnvalue
    (bind _returnvalue_2 (CallFunction|GetTargetwithMaxPriority (Variables|Default|GetTargetsForAbility) true))
    (Default|AttackTargetSERVER (Variables|Default|GetControlledUnit) _returnvalue_2 true)
    (else
      (bind _returnvalue_3 (CallFunction|GetTargetwithMaxPriority (Variables|Default|GetAvailableTargets) false))
      (Default|AttackTargetSERVER (Variables|Default|GetControlledUnit) _returnvalue_3 false))))

(fn ConstructionScript
  (|CallParentFunction))

(fn GetTargetwithMaxPriority
  (params (Targets :type Array%20of%20BP%20Hero%20Base%20Object%20References) (bUseAbility :type Boolean))
  (for _array_element Targets
    (bind _finalpriority (CallFunction|CalculateEffectivnessOfAttack _array_element bUseAbility))
    (if (> _finalpriority (LocalVariables|GetL_MaxPriority))
      (LocalVariables|SetL_MaxPriority _finalpriority)
      (LocalVariables|SetL_Unit _array_element)))
  (return (LocalVariables|GetL_Unit)))