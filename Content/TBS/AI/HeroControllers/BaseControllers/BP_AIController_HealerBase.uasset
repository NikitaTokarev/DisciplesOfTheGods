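; Base AI controller for healer units in the turn-based game, choosing which available target to heal or defending otherwise.
; Target selection skips units at full health and scores injured ones by base priority plus a bonus that grows as health percentage drops.
; The top-scoring unit goes to the controlled unit's server attack call without using an ability; with no valid target, the unit defends.
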(event EventBeginPlay)

(event EventSelectBestAction
  (bind _returnvalue (CallFunction|GetTargetwithMaxPriority (Variables|Default|GetAvailableTargets) false))
  (Utilities|IsValid _returnvalue
    (:Is%20Valid
      (Default|AttackTargetSERVER (Variables|Default|GetControlledUnit) _returnvalue false))
    (:Is%20Not%20Valid
      (Default|DefendSERVER (Variables|Default|GetControlledUnit)))))

(fn ConstructionScript
  (|CallParentFunction))

(fn GetTargetwithMaxPriority
  (params (Targets :type Array%20of%20BP%20Hero%20Base%20Object%20References) (bUseAbility :type Boolean))
  (for _array_element Targets
    (bind (_fullhp _returnvalue) (CallFunction|CalcPriorityforHealing _array_element))
    (if (not _fullhp)
      (if (> _returnvalue (LocalVariables|GetL_MaxPriority))
        (LocalVariables|SetL_MaxPriority _returnvalue)
        (LocalVariables|SetL_Unit _array_element))))
  (return (LocalVariables|GetL_Unit)))

(fn CalcPriorityforHealing
  (params (Unit :type BP%20Hero%20Base%20Object%20Reference))
  (bind _returnvalue (Default|GetUnitBasePriority Unit))
  (if (Default|IsUnitInjured Unit)
    (return false (+ _returnvalue (Math|Float|Round (* _returnvalue (- 1.5 (Default|GetUnitPercentHealth Unit))))))
    (else
      (return true -999))))